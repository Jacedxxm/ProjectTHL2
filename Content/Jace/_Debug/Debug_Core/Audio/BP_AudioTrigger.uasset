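; BP_AudioTrigger is a box trigger actor that signals sound changes through event dispatchers as the player enters or leaves it.
; It caches the player reference on BeginPlay, then broadcasts OnNewSoundTrigger with NewSound on overlap begin and OnNewSoundExitTrigger on overlap end.
; Each overlap path has its own DoOnce ahead of the player check, so the first overlap by any actor uses up that path.
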(event OnComponentBeginOverlap(Box)
  (params (OverlappedComponent :type Primitive%20Component%20Object%20Reference) (OtherActor :type Actor%20Object%20Reference) (OtherComp :type Primitive%20Component%20Object%20Reference) (OtherBodyIndex :type Integer) (bFromSweep :type Boolean) (SweepResult :type Hit%20Result%20Structure%20%28by%20ref%29))
  (Utilities|FlowControl|DoOnce false
    (:Completed
      (if (== OtherActor (Variables|Default|GetPlayerCharacter))
        (Default|CallOnNewSoundTrigger (Variables|Default|GetNewSound))))))

(event OnComponentEndOverlap(Box)
  (params (OverlappedComponent :type Primitive%20Component%20Object%20Reference) (OtherActor :type Actor%20Object%20Reference) (OtherComp :type Primitive%20Component%20Object%20Reference) (OtherBodyIndex :type Integer))
  (Utilities|FlowControl|DoOnce false
    (:Completed
      (if (== OtherActor (Variables|Default|GetPlayerCharacter))
        (Default|CallOnNewSoundExitTrigger)))))

(event EventBeginPlay
  (bind _playerref (CallFunction|GetPlayerReference))
  (Variables|Default|SetPlayerCharacter _playerref))

(fn ConstructionScript)