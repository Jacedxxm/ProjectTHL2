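; BP_SoundTrigger is a trigger volume that plays an environment sound when the player enters its box.
; On BeginPlay it caches the player reference, then compares each overlapping actor against it.
; An IsRetriggerable flag selects between playing EnvSound on every entry or only once through a DoOnce.
; The sound plays as non-spatialized 2D audio.
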(event OnComponentBeginOverlap(Box)
  (params (OverlappedComponent :type Primitive%20Component%20Object%20Reference) (OtherActor :type Actor%20Object%20Reference) (OtherComp :type Primitive%20Component%20Object%20Reference) (OtherBodyIndex :type Integer) (bFromSweep :type Boolean) (SweepResult :type Hit%20Result%20Structure%20%28by%20ref%29))
  (bind _envsound (Variables|Default|GetEnvSound))
  (if (== OtherActor (Variables|Default|GetPlayer%20Ref))
    (if (Variables|Default|GetbIsRetriggerable)
      (Audio|PlaySound2D _envsound 1.0 1.0 0.0 0 0)
      (else
        (Utilities|FlowControl|DoOnce false
          (:Completed
            (Audio|PlaySound2D _envsound 1.0 1.0 0.0 0 0)))))))

(event EventBeginPlay
  (bind _playerref (CallFunction|GetPlayerReference))
  (Variables|Default|SetPlayer%20Ref _playerref))

(fn ConstructionScript)