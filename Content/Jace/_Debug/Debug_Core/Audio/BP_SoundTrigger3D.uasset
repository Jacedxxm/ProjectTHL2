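; BP_SoundTrigger3D is a trigger volume that plays a 3D environment sound when the player character enters its box.
; The sound plays at the location of a referenced actor, ActorRef.
; IsRetriggerable selects between playing on every overlap and playing once through a DoOnce gate.
; BeginPlay caches a player reference, but the overlap check compares against player character 0 directly.
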(event OnComponentBeginOverlap(Box)
  (params (OverlappedComponent :type Primitive%20Component%20Object%20Reference) (OtherActor :type Actor%20Object%20Reference) (OtherComp :type Primitive%20Component%20Object%20Reference) (OtherBodyIndex :type Integer) (bFromSweep :type Boolean) (SweepResult :type Hit%20Result%20Structure%20%28by%20ref%29))
  (bind _envsound (Variables|Default|GetEnvSound))
  (bind _actorref (Variables|Default|GetActorRef))
  (bind _returnvalue (Transformation|GetActorLocation _actorref))
  (if (== OtherActor (Game|GetPlayerCharacter 0))
    (if (Variables|Default|GetbIsRetriggerable)
      (Audio|PlaySoundatLocation _envsound _returnvalue "0, 0, 0" 1.0 1.0 0.0 0 0 0 0)
      (else
        (Utilities|FlowControl|DoOnce false
          (:Completed
            (Audio|PlaySoundatLocation _envsound _returnvalue "0, 0, 0" 1.0 1.0 0.0 0 0 0 0)))))))

(event EventBeginPlay
  (bind _playerref (CallFunction|GetPlayerReference))
  (Variables|Default|SetPlayer%20Ref _playerref))

(fn ConstructionScript)