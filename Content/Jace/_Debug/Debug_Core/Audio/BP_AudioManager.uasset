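; Debug audio manager Blueprint that switches and plays sounds on a single audio component in response to audio triggers.
; On BeginPlay it binds to the new-sound and exit events of every trigger in its AudioTriggers array.
; A new-sound trigger stops playback and assigns the sound, and the exit trigger starts playing it from the beginning.
; Both steps print colored debug strings to the screen.
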(event Custom|PlaySound
  (Audio|Components|Audio|Play (Variables|Default|GetAudio) 0.0)
  (Development|PrintString "Hello" true true "(R=1.000000,G=0.850628,B=0.000000,A=1.000000)"))

(event Custom|StopSound
  (Audio|Components|Audio|Stop (Variables|Default|GetAudio)))

(event Custom|SetNewSound
  (params (SoundToPlay :type Sound%20Cue%20Object%20Reference))
  (CallFunction|StopSound)
  (Audio|Components|Audio|SetSound (Variables|Default|GetAudio) SoundToPlay)
  (Development|PrintString "Hello" true true "(R=0.000000,G=0.016063,B=1.000000,A=1.000000)"))

(event EventBeginPlay
  (for _array_element (Variables|Default|GetAudioTriggers)
    (EventDispatchers|BindEventtoOnNewSoundTrigger _array_element (delegate Custom|SetNewSound))
    (EventDispatchers|BindEventtoOnNewSoundExitTrigger _array_element (delegate Custom|PlaySound))))

(fn ConstructionScript)