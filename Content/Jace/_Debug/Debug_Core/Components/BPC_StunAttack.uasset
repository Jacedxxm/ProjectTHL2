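; BPC_StunAttack is a debug-core component that stuns the enemy in the camera's line of sight.
; TryToStun runs a Visibility line trace between camera-derived points limited by a maximum distance, with debug drawing.
; A hit BP_BaseEnemy has its mesh switched to simulated physics with the Ragdoll collision profile, and its AI controller unpossesses it.
; The file contains no recovery from this state.
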(event Custom|TryToStun
  (params (StunAttackMaxDistance :type Float%20%28double-precision%29))
  (bind (_startpoint _endpoint) (CallFunction|FindCameraTracePoints StunAttackMaxDistance))
  (bind _outhit (Collision|LineTraceByChannel _startpoint _endpoint "TraceTypeQuery1" false 0 "ForOneFrame"))
  (bind _asbp_base_enemy (Utilities|Casting|CastToBP_BaseEnemy (.HitActor (Collision|BreakHitResult _outhit))))
  (Utilities|IsValid _asbp_base_enemy
    (:Is%20Valid
      (Physics|SetSimulatePhysics (Variables|/Script/Engine.Character|GetMesh _asbp_base_enemy) true)
      (Collision|SetCollisionProfileName (Variables|/Script/Engine.Character|GetMesh _asbp_base_enemy) "Ragdoll" true :!class /Script/Engine.PrimitiveComponent)
      (Utilities|IsValid (.HitActor (Collision|BreakHitResult _outhit))
        (:Is%20Valid
          (Pawn|UnPossess (AI|GetAIController (.HitActor (Collision|BreakHitResult _outhit)))))))))

(event EventBeginPlay)