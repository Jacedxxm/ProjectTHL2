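; BPC_DebugComponent is a debug component meant to draw a debug sphere at its owner's location.
; BeginPlay starts a looping two-second timer that targets SetDebug by function name and stores the handle in Timer.
; SetDebug draws the sphere only when the Debug flag is set, using radius, duration, thickness and color inputs, which the name-based timer cannot supply.
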(event Custom|DebugCollisionTimer
  (bind _returnvalue (Utilities|Time|SetTimerbyFunctionName 0 "SetDebug" 2.0 true))
  (Variables|Default|SetTimer _returnvalue))

(event EventBeginPlay
  (CallFunction|DebugCollisionTimer))

(fn SetDebug
  (params (Radius :type Float%20%28single-precision%29) (Duration :type Float%20%28single-precision%29) (Thickness :type Float%20%28single-precision%29) (LineColor :type Linear%20Color%20Structure))
  (if (Variables|Default|GetbDebug)
    (Rendering|Debug|DrawDebugSphere (Transformation|GetActorLocation (Components|GetOwner)) Radius 12 LineColor Duration Thickness)
    (return)))