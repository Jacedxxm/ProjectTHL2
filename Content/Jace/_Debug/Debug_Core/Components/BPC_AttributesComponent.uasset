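; Actor component that stores named gameplay attributes in a map of attribute structs, each with a current, minimum and maximum value.
; SetAttribute assigns a value and ModifyAttribute adds a delta, both clamping to that attribute's range, writing the struct back to the map and returning the clamped result.
; GetAttributeValue reads the current value.
; All three act only when the name exists in the map, and BeginPlay is empty.
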(event EventBeginPlay)

(fn SetAttribute
  (params (NewAttributeValue :type Float%20%28double-precision%29) (AttributeName :type Name))
  (bind _attributes (Variables|Default|GetAttributes))
  (bind (_value _returnvalue) (Utilities|Map|Find _attributes AttributeName))
  (bind (_minvalue _currentvalue _maxvalue) (Utilities|Struct|BreakST_Attribute _value))
  (bind _returnvalue_2 (Math|Float|Clamp(Float) NewAttributeValue _minvalue _maxvalue))
  (if _returnvalue
    (bind _structout (Utilities|Struct|SetmembersinST_Attribute _value _returnvalue_2))
    (Utilities|Map|Add _attributes AttributeName _structout)
    (return _returnvalue_2)))

(fn GetAttributeValue
  (params (AttributeName :type Name))
  (bind _attributes (Variables|Default|GetAttributes))
  (bind (_value _returnvalue) (Utilities|Map|Find _attributes AttributeName))
  (if _returnvalue
    (return (.currentvalue _value))))

(fn ModifyAttribute
  (params (ModifiyAmount :type Float%20%28double-precision%29) (AttributeName :type Name))
  (bind _attributes (Variables|Default|GetAttributes))
  (bind (_value _returnvalue) (Utilities|Map|Find _attributes AttributeName))
  (bind (_minvalue _currentvalue _maxvalue) (Utilities|Struct|BreakST_Attribute _value))
  (bind _returnvalue_2 (+ ModifiyAmount _currentvalue))
  (bind _returnvalue_3 (Math|Float|Clamp(Float) _returnvalue_2 _minvalue _maxvalue))
  (if _returnvalue
    (bind _structout (Utilities|Struct|SetmembersinST_Attribute _value _returnvalue_3))
    (Utilities|Map|Add _attributes AttributeName _structout)
    (return _returnvalue_3)))