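; Debug actor component that gives its owner a cooldown-limited stun attack against enemies.
; TryToStun disables the ability, starts a cooldown timer and line-traces on Visibility between camera trace points at the given distance.
; A hit BP_BaseEnemy is ragdolled through mesh physics, its AI controller unpossesses it and its capsule collision turns off, with no recovery in this graph.
; ResetCooldown clears the timer and re-enables the ability.
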(event Custom|TryToStun
  (params (StunAttackMaxDistance :type Float%20%28double-precision%29))
  (bind (_startpoint _endpoint) (CallFunction|FindCameraTracePoints StunAttackMaxDistance))
  (Variables|Default|SetbCanUseAbility false)
  ;[0.004612 0.15 0.1455 0.5] Start Cooldown
  (bind _returnvalue (Utilities|Time|SetTimerbyEvent (EventDispatchers|CreateEvent :!event Custom|ResetCooldown) (Variables|Default|GetAbilityCooldown)))
  (Variables|Default|SetCooldownTimer _returnvalue)
  ;[0.03382 0.03314 0.15 0.5] Check Target
  (bind _outhit (Collision|LineTraceByChannel _startpoint _endpoint "TraceTypeQuery1" false 0 "ForOneFrame"))
  (bind _asbp_base_enemy (Utilities|Casting|CastToBP_BaseEnemy (.HitActor (Collision|BreakHitResult _outhit))))
  (Utilities|IsValid _asbp_base_enemy
    (:Is%20Valid
      ;[0.15 0.02109 0.02109 0.5] Stun Enemy
      (Physics|SetSimulatePhysics (Variables|/Script/Engine.Character|GetMesh _asbp_base_enemy) true)
      (Collision|SetCollisionProfileName (Variables|/Script/Engine.Character|GetMesh _asbp_base_enemy) "Ragdoll" true :!class /Script/Engine.PrimitiveComponent)
      (Utilities|IsValid (.HitActor (Collision|BreakHitResult _outhit))
        (:Is%20Valid
          (Pawn|UnPossess (AI|GetAIController (.HitActor (Collision|BreakHitResult _outhit))))
          (Collision|SetCollisionEnabled (Variables|/Script/Engine.Character|GetCapsuleComponent _asbp_base_enemy) "NoCollision"))))))

(event Custom|ResetCooldown
  ;[0.1484 0.15 0.04088 0.5] Reset Cooldown
  (Utilities|Time|ClearandInvalidateTimerbyHandle (Variables|Default|GetCooldownTimer))
  (Variables|Default|SetbCanUseAbility true))