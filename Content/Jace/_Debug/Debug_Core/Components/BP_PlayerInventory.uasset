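; Debug player inventory Blueprint that tracks rifle and magazine ammo counts.
; Pressing the debug M key adds a fixed amount of rifle ammo.
; Tick prints both counts on screen and clamps magazine ammo to its maximum.
; The rifle ammo reset and clamp are disconnected, so that count can grow past its unused maximum.
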(event EventBeginPlay)

(event EventTick
  (params (DeltaSeconds :type Float%20%28single-precision%29))
  (Development|PrintString (Utilities|String|ToString(Integer) (Variables|Default|GetCurrentMagazineAmmo)) true true "(R=0.000000,G=0.660000,B=1.000000,A=1.000000)" DeltaSeconds)
  (Variables|Default|SetCurrentMagazineAmmo (Math|Integer|Clamp(Integer) (Variables|Default|GetCurrentMagazineAmmo) 0 (Variables|Default|GetMaxMagazineAmmo)))
  (Development|PrintString (Utilities|String|ToString(Integer) (Variables|Default|GetCurrentRifleAmmo)) true true "(R=1.000000,G=0.000000,B=0.024480,A=1.000000)" 0.0))

(event Input|KeyboardEvents|DebugKeyM
  (params (Key :type Key%20Structure :default "None") (ActionValue :type Input%20Action%20Value%20Structure))
  (:Pressed
    (Variables|Default|SetCurrentRifleAmmo (+ (Variables|Default|GetCurrentRifleAmmo) 10))))