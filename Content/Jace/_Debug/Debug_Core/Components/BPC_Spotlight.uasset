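; Spotlight component that acts as a toggleable flashlight with a limited, self-recharging energy supply.
; While lit, it lerps its rotation toward the camera view and drains energy, switching off at zero.
; While off, it recharges, then disables its tick and plays a shutter sound after a short delay once full.
; Debug helpers print the energy value and let the P key set it low.
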(event Custom|Toggle
  ;[0.15 0.15 0.15 0.5] Toggle  Flashlight
  (if (and (not (Variables|FlashlightState|GetbIsOn)) (> (Variables|Energy|GetCurrentEnergy) 0.0))
    (CallFunction|ActivateFlashlight)
    (else
      (CallFunction|DeactivateFlashlight))))

(event Custom|ActivateFlashlight
  ;[0.15 0.15 0.15 0.5] Activate/Deactivate
  (Components|Tick|SetComponentTickEnabled true)
  (Rendering|Components|Light|SetIntensity 1e+04)
  (Variables|FlashlightState|SetbIsOn true))

(event Custom|DeactivateFlashlight
  ;[0.15 0.15 0.15 0.5] Activate/Deactivate
  (Rendering|Components|Light|SetIntensity 0.0)
  (Variables|FlashlightState|SetbIsOn false))

(event EventBeginPlay
  (CallFunction|SetEnergy)
  (Components|Tick|SetComponentTickEnabled false)
  (bind _playerref (CallFunction|GetPlayerReference))
  (Variables|Default|SetPlayerCharacter _playerref))

(event EventTick
  (params (DeltaSeconds :type Float%20%28single-precision%29))
  ;[0.15 0.15 0.15 0.5] Flashlight Energy loop
  (if (Variables|FlashlightState|GetbIsOn)
    (Development|PrintString (Utilities|String|ToString(Float) (Variables|Energy|GetCurrentEnergy)) true true "(R=0.000000,G=0.660000,B=1.000000,A=1.000000)" DeltaSeconds)
    (Utilities|CheckifNotOutOfEnergy
      (:True
        (CallFunction|DeactivateFlashlight))
      (:False
        (Transformation|SetWorldRotation (CallFunction|FollowCaemra) false false)
        (if (Variables|FlashlightState|GetbIsOn)
          (Variables|Energy|SetCurrentEnergy (CallFunction|ConsumeEnergy)))))
    (else
      (bind _output_get (Variables|Energy|SetCurrentEnergy (CallFunction|RecoverEnergy)))
      (if (== _output_get (Variables|Energy|GetMaxEnergy))
        (Components|Tick|SetComponentTickEnabled false)
        (Utilities|FlowControl|Delay 0.2)
        (Audio|PlaySound2D "/Engine/VREditor/Sounds/UI/Camera_Shutter.Camera_Shutter" 1.0 1.0 0.0 0 0)))))

(event Input|KeyboardEvents|DebugKeyP
  (params (Key :type Key%20Structure :default "None") (ActionValue :type Input%20Action%20Value%20Structure))
  ;[0.15 0 0.09705 0.5] Flashlight Debug
  (:Pressed
    (Variables|Energy|SetCurrentEnergy 5.0)))

(fn FollowCaemra
  (return (Math|Rotator|Lerp(Rotator) (Transformation|GetWorldRotation) (Utilities|Struct|BreakMinimalViewInfo (Class|SequenceCameraShakeTestUtil|GetCameraCachePOV (Game|GetPlayerController 0))) (* (Utilities|Time|GetWorldDeltaSeconds) (Variables|Orientation|GetCameraFollowSpeed)) true)))

(fn SetEnergy
  (Variables|Energy|SetCurrentEnergy (Math|Float|Clamp(Float) (Variables|Energy|GetCurrentEnergy) 0.0 (Variables|Energy|GetMaxEnergy))))

(fn ConsumeEnergy
  (return (Math|Float|Clamp(Float) (- (Variables|Energy|GetCurrentEnergy) (* (Utilities|Time|GetWorldDeltaSeconds) (Variables|Energy|GetEnergyCost))) 0.0 (Variables|Energy|GetMaxEnergy))))

(fn RecoverEnergy
  (bind _returnvalue (Utilities|Time|GetWorldDeltaSeconds))
  (bind _maxenergy (Variables|Energy|GetMaxEnergy))
  (bind _currentenergy (Variables|Energy|GetCurrentEnergy))
  (bind _energyrecovringvalue (Variables|Energy|GetEnergyRecovringValue))
  (bind _returnvalue_2 (* _returnvalue _energyrecovringvalue))
  (bind _returnvalue_3 (+ _currentenergy _returnvalue_2))
  (bind _returnvalue_4 (Math|Float|Clamp(Float) _returnvalue_3 0.0 _maxenergy))
  (Development|PrintString (Utilities|String|ToString(Float) _returnvalue_4) true true "(R=0.000000,G=0.660000,B=1.000000,A=1.000000)" 0.0)
  (return _returnvalue_4))