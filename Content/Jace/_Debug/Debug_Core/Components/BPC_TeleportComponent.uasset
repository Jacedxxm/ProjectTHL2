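; Player component that adds a hold-to-aim, release-to-teleport ability to BP_PlayerCharacter_VortigauntTest.
; While aiming, Tick chains line and sphere traces to place the target marker on the ground or atop obstacles, showing a can't-teleport effect when no floor is found.
; Mouse wheel shifts the trace points to change range.
; Release briefly disables input, collision and mesh visibility, then calls the character's TeleportTime with effects and sound.
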(event Input|EnhancedActionEvents|EnhancedInputActionIA_TeleportActivation
  (params (ActionValue :type Boolean) (ElapsedSeconds :type Float%20%28double-precision%29) (TriggeredSeconds :type Float%20%28double-precision%29) (InputAction :type Input%20Action%20Object%20Reference :default "/Game/FirstPerson/Input/Actions/IA_TeleportActivation.IA_TeleportActivation"))
  (bind _returnvalue (Game|GetPlayerController 0))
  (bind _returnvalue_2 (Game|GetPlayerController 0))
  (bind _playercharacter (Variables|Default|GetPlayerCharacter))
  (bind _playercharacter_2 (Variables|Default|GetPlayerCharacter))
  (bind _playercharacter_3 (Variables|Default|GetPlayerCharacter))
  (bind _playercharacter_4 (Variables|Default|GetPlayerCharacter))
  (bind _playercharacter_5 (Variables|Default|GetPlayerCharacter))
  (bind _charactermovement (Variables|/Script/Engine.Character|GetCharacterMovement _playercharacter_5))
  ;[0.3121 0.1751 0.3281 0.5] Teleport Ability
  (:Started
    (bind _returnvalue_3 (Audio|SpawnSound2D "/Game/Jace/_Debug/Debug_Core/Audio/SFX_TeleportHolding.SFX_TeleportHolding" 1.0 1.0 0.0 0))
    (Variables|Default|SetHoldingSound _returnvalue_3)
    ;;[0.07679 0.15 0.07518 0.5] Ability Activation
    (bind _playercharacter_6 (Variables|Default|GetPlayerCharacter)
      (:then
        (if (Variables|/Game/FirstPerson/Blueprints/BP_PlayerCharacter_VortigauntTest.BP_PlayerCharacter_VortigauntTest_C|GetbIsTeleporting _playercharacter_6)
          (bind _output_get (Variables|/Game/FirstPerson/Blueprints/BP_PlayerCharacter_VortigauntTest.BP_PlayerCharacter_VortigauntTest_C|SetbIsTeleporting _playercharacter_6 false))
          (Default|SetTeleportFX _playercharacter _output_get)
          (else
            (bind _output_get_2 (Variables|/Game/FirstPerson/Blueprints/BP_PlayerCharacter_VortigauntTest.BP_PlayerCharacter_VortigauntTest_C|SetbIsTeleporting _playercharacter_6 true))
            (Default|SetTeleportFX _playercharacter _output_get_2))))
      (:else)))
  (:Completed
    (bind _holdingsound (Variables|Default|GetHoldingSound)
      (:then
        (Audio|Components|Audio|Stop _holdingsound)
        (bind _playercharacter_7 (Variables|Default|GetPlayerCharacter)
          (:then
            (if (Variables|/Game/FirstPerson/Blueprints/BP_PlayerCharacter_VortigauntTest.BP_PlayerCharacter_VortigauntTest_C|GetbIsTeleporting _playercharacter_7)
              (if (Variables|/Game/FirstPerson/Blueprints/BP_PlayerCharacter_VortigauntTest.BP_PlayerCharacter_VortigauntTest_C|GetbCanTeleport _playercharacter_7)
                (Variables|/Game/FirstPerson/Blueprints/BP_PlayerCharacter_VortigauntTest.BP_PlayerCharacter_VortigauntTest_C|SetbIsTeleporting _playercharacter_4 false)
                (Effects|SpawnEmitteratLocation "/Game/FXVarietyPack/Particles/P_ky_hit1.P_ky_hit1" (Transformation|GetActorLocation _playercharacter_4))
                (Rendering|SetVisibility (Variables|/Game/FirstPerson/Blueprints/BP_FirstPersonCharacter.BP_FirstPersonCharacter_C|GetFirstPersonMesh _playercharacter_5) false false)
                (Components|Movement|StopMovementImmediately _charactermovement)
                (Input|DisableInput _returnvalue_2 _returnvalue_2)
                (Pawn|Components|CharacterMovement|SetMovementMode _charactermovement "MOVE_Flying" 0)
                (Collision|SetCollisionEnabled (Variables|/Script/Engine.Character|GetCapsuleComponent (Variables|Default|GetPlayerCharacter)) "NoCollision")
                (Utilities|FlowControl|Delay 0.5)
                (Default|SetTeleportFX _playercharacter_3 false)
                (bind _output_get_3 (Variables|Default|SetTeleportLocation (Transformation|GetWorldLocation (Variables|/Game/FirstPerson/Blueprints/BP_PlayerCharacter_VortigauntTest.BP_PlayerCharacter_VortigauntTest_C|GetTeleportTargetPosition_0 _playercharacter_3))))
                (Default|TeleportTime (Variables|Default|GetPlayerCharacter) _output_get_3)
                (Audio|PlaySound2D "/Game/Jace/_Debug/Debug_Core/Audio/SFX_Teleport.SFX_Teleport" 1.0 1.0 0.0 0 0)
                (Effects|SpawnEmitteratLocation "/Game/FXVarietyPack/Particles/P_ky_hit1.P_ky_hit1" (Transformation|GetActorLocation (Variables|Default|GetPlayerCharacter)))
                (Rendering|SetVisibility (Variables|/Game/FirstPerson/Blueprints/BP_FirstPersonCharacter.BP_FirstPersonCharacter_C|GetFirstPersonMesh _playercharacter_2) true false)
                (Input|EnableInput _returnvalue _returnvalue)
                (Pawn|Components|CharacterMovement|SetMovementMode (Variables|/Script/Engine.Character|GetCharacterMovement _playercharacter_2) "MOVE_Walking" 0)
                (Collision|SetCollisionEnabled (Variables|/Script/Engine.Character|GetCapsuleComponent (Variables|Default|GetPlayerCharacter)) "QueryAndPhysics"))))
          (:else)))
      (:else))))

(event EventBeginPlay
  ;[0 0.01127 0.15 0.5] Setup
  (bind _asbp_player_character_vortigaunt_test (Utilities|Casting|CastToBP_PlayerCharacter_VortigauntTest (Game|GetPlayerCharacter 0)))
  (Variables|Default|SetPlayerCharacter _asbp_player_character_vortigaunt_test))

(event EventTick
  (params (DeltaSeconds :type Float%20%28single-precision%29))
  (bind (_teleportstartlocation _teleportenddistance) (CallFunction|GetTeleportPointsLocations))
  (bind _playercharacter (Variables|Default|GetPlayerCharacter))
  (bind _playercharacter_2 (Variables|Default|GetPlayerCharacter))
  (bind _playercharacter_3 (Variables|Default|GetPlayerCharacter))
  (bind _playercharacter_4 (Variables|Default|GetPlayerCharacter))
  (bind _playercharacter_5 (Variables|Default|GetPlayerCharacter))
  (bind _playercharacter_6 (Variables|Default|GetPlayerCharacter))
  (bind _playercharacter_7 (Variables|Default|GetPlayerCharacter))
  (bind _downtrace_0 (Variables|/Game/FirstPerson/Blueprints/BP_PlayerCharacter_VortigauntTest.BP_PlayerCharacter_VortigauntTest_C|GetDownTrace_0 _playercharacter_2))
  (bind _movecube_0 (Variables|/Game/FirstPerson/Blueprints/BP_PlayerCharacter_VortigauntTest.BP_PlayerCharacter_VortigauntTest_C|GetMoveCube_0 _playercharacter_3))
  (bind _begintrace_0 (Variables|/Game/FirstPerson/Blueprints/BP_PlayerCharacter_VortigauntTest.BP_PlayerCharacter_VortigauntTest_C|GetBeginTrace_0 _playercharacter_5))
  (bind _movecube_0_2 (Variables|/Game/FirstPerson/Blueprints/BP_PlayerCharacter_VortigauntTest.BP_PlayerCharacter_VortigauntTest_C|GetMoveCube_0 _playercharacter_7))
  (bind _cantteleportfx_0 (Variables|/Game/FirstPerson/Blueprints/BP_PlayerCharacter_VortigauntTest.BP_PlayerCharacter_VortigauntTest_C|GetCantTeleportFX_0 _playercharacter_6))
  (bind _downtrace_0_2 (Variables|/Game/FirstPerson/Blueprints/BP_PlayerCharacter_VortigauntTest.BP_PlayerCharacter_VortigauntTest_C|GetDownTrace_0 _playercharacter))
  (bind _returnvalue (Transformation|GetWorldLocation _movecube_0))
  (bind _returnvalue_2 (Transformation|GetWorldLocation _downtrace_0))
  (bind _returnvalue_3 (Transformation|GetWorldLocation _downtrace_0_2))
  (bind _returnvalue_4 (Transformation|GetWorldLocation _movecube_0_2))
  (bind _returnvalue_5 (Math|Vector|GetForwardVector _movecube_0_2))
  (bind _returnvalue_6 (Transformation|GetWorldLocation _begintrace_0))
  (bind _returnvalue_7 (* _returnvalue_5 5e+02))
  (bind _returnvalue_8 (+ _returnvalue_4 _returnvalue_7))
  (bind _returnvalue_9 (+ _returnvalue_4 _returnvalue_7))
  (bind _playercharacter_8 (Variables|Default|GetPlayerCharacter)
    (:then
      (if (Variables|/Game/FirstPerson/Blueprints/BP_PlayerCharacter_VortigauntTest.BP_PlayerCharacter_VortigauntTest_C|GetbIsTeleporting _playercharacter_8)
        (Transformation|SetWorldRotation (Variables|/Game/FirstPerson/Blueprints/BP_PlayerCharacter_VortigauntTest.BP_PlayerCharacter_VortigauntTest_C|GetCube_0 _playercharacter_8) (Math|Rotator|MakeRotator (.roll (Pawn|GetBaseAimRotation _playercharacter_8)) 0.0 (.yaw (Pawn|GetBaseAimRotation _playercharacter_8))) false false)
        (bind _outhit (Collision|LineTraceByChannel _teleportstartlocation _teleportenddistance "TraceTypeQuery1" false 0 "None"))
        (if (.bBlockingHit (Collision|BreakHitResult _outhit))
          (Transformation|SetWorldLocation _movecube_0 (.ImpactPoint (Collision|BreakHitResult _outhit)) false false)
          (bind _outhit_2 (Collision|LineTraceByChannel _returnvalue (+ _returnvalue (* (Math|Vector|GetForwardVector _movecube_0) 7e+01)) "TraceTypeQuery1" false 0 "None"))
          (Transformation|SetWorldLocation (Variables|/Game/FirstPerson/Blueprints/BP_PlayerCharacter_VortigauntTest.BP_PlayerCharacter_VortigauntTest_C|GetDownTrace_0 (Variables|Default|GetPlayerCharacter)) (Math|Vector|MakeVector (.x (.TraceEnd (Collision|BreakHitResult _outhit_2))) (.y (.TraceEnd (Collision|BreakHitResult _outhit_2))) (+ (.z (.TraceEnd (Collision|BreakHitResult _outhit_2))) 5e+02)) false false)
          (bind _outhit_3 (Collision|LineTraceByChannel (Transformation|GetWorldLocation _downtrace_0) (Math|Vector|MakeVector (.x _returnvalue_2) (.y _returnvalue_2) (+ (.z _returnvalue_2) 3e+01)) "TraceTypeQuery1" false 0 "ForOneFrame"))
          (if (.bBlockingHit (Collision|BreakHitResult _outhit_3))
            (Collision|LineTraceByChannel _returnvalue_4 _returnvalue_8 "TraceTypeQuery1" false 0 "None")
            (bind _outhit_4 (Collision|LineTraceByChannel _returnvalue_8 (Math|Vector|MakeVector (.x _returnvalue_9) (.y _returnvalue_9) -5e+02) "TraceTypeQuery1" false 0 "None"))
            (else
              (bind _outhit_5 (Collision|SphereTraceByChannel (Transformation|GetWorldLocation (Variables|/Game/FirstPerson/Blueprints/BP_PlayerCharacter_VortigauntTest.BP_PlayerCharacter_VortigauntTest_C|GetDownTrace_0 (Variables|Default|GetPlayerCharacter))) (Math|Vector|MakeVector (.x _returnvalue_3) (.y _returnvalue_3) -5e+02) 6e+01 "TraceTypeQuery1" false 0 "None"))
              (Default|SetTeleportFX _playercharacter_4 true)
              (Transformation|SetWorldLocation (Variables|/Game/FirstPerson/Blueprints/BP_PlayerCharacter_VortigauntTest.BP_PlayerCharacter_VortigauntTest_C|GetTeleportTargetPosition_0 _playercharacter_4) (.ImpactPoint (Collision|BreakHitResult _outhit_5)) false false)
              (Variables|/Game/FirstPerson/Blueprints/BP_PlayerCharacter_VortigauntTest.BP_PlayerCharacter_VortigauntTest_C|SetbCanTeleport (Variables|Default|GetPlayerCharacter) true)
              (Rendering|SetVisibility (Variables|/Game/FirstPerson/Blueprints/BP_PlayerCharacter_VortigauntTest.BP_PlayerCharacter_VortigauntTest_C|GetCantTeleportFX_0 (Variables|Default|GetPlayerCharacter)) false false)))
          (else
            (bind _outhit_6 (Collision|LineTraceByChannel (Transformation|GetWorldLocation (Variables|/Game/FirstPerson/Blueprints/BP_PlayerCharacter_VortigauntTest.BP_PlayerCharacter_VortigauntTest_C|GetBeginTrace_0 (Variables|Default|GetPlayerCharacter))) (Math|Vector|MakeVector (.x _returnvalue_6) (.y _returnvalue_6) (- (.z _returnvalue_6) 5e+03)) "TraceTypeQuery1" false 0 "None"))
            (if (.bBlockingHit (Collision|BreakHitResult _outhit_6))
              (CallFunction|SetTeleportFXLocation (.ImpactPoint (Collision|BreakHitResult _outhit_6)))
              (Rendering|SetVisibility (Variables|/Game/FirstPerson/Blueprints/BP_PlayerCharacter_VortigauntTest.BP_PlayerCharacter_VortigauntTest_C|GetTeleportTargetPosition_0 (Variables|Default|GetPlayerCharacter)) true false)
              (Variables|/Game/FirstPerson/Blueprints/BP_PlayerCharacter_VortigauntTest.BP_PlayerCharacter_VortigauntTest_C|SetbCanTeleport (Variables|Default|GetPlayerCharacter) true)
              (Rendering|SetVisibility (Variables|/Game/FirstPerson/Blueprints/BP_PlayerCharacter_VortigauntTest.BP_PlayerCharacter_VortigauntTest_C|GetCantTeleportFX_0 (Variables|Default|GetPlayerCharacter)) false false)
              (else
                (Rendering|SetVisibility (Variables|/Game/FirstPerson/Blueprints/BP_PlayerCharacter_VortigauntTest.BP_PlayerCharacter_VortigauntTest_C|GetTeleportTargetPosition_0 (Variables|Default|GetPlayerCharacter)) false false)
                (Variables|/Game/FirstPerson/Blueprints/BP_PlayerCharacter_VortigauntTest.BP_PlayerCharacter_VortigauntTest_C|SetbCanTeleport (Variables|Default|GetPlayerCharacter) false)
                (Rendering|SetVisibility _cantteleportfx_0 true false)
                (Transformation|SetWorldLocation _cantteleportfx_0 (Math|Vector|MakeVector (.x (.TraceEnd (Collision|BreakHitResult _outhit_6))) (.y (.TraceEnd (Collision|BreakHitResult _outhit_6))) (+ (.z (.TraceEnd (Collision|BreakHitResult _outhit_6))) 4.5e+02)) false false)))))))
    (:else)))

(event Input|MouseEvents|MouseWheelDown
  (params (Key :type Key%20Structure :default "None"))
  (bind _playercharacter (Variables|Default|GetPlayerCharacter))
  (bind _downtrace_0 (Variables|/Game/FirstPerson/Blueprints/BP_PlayerCharacter_VortigauntTest.BP_PlayerCharacter_VortigauntTest_C|GetDownTrace_0 _playercharacter))
  (bind _begintrace_0 (Variables|/Game/FirstPerson/Blueprints/BP_PlayerCharacter_VortigauntTest.BP_PlayerCharacter_VortigauntTest_C|GetBeginTrace_0 _playercharacter))
  (bind _relativelocation (Variables|/Script/Engine.SceneComponent|GetRelativeLocation _begintrace_0))
  (bind _relativelocation_2 (Variables|/Script/Engine.SceneComponent|GetRelativeLocation _downtrace_0))
  ;[0.15 0.1159 0.000808 0.5] Mouse Wheele Distance Teleport Modifier
  (:Pressed
    (Transformation|SetRelativeLocation _begintrace_0 (Math|Vector|MakeVector (- (.x _relativelocation) 2e+02) (.y _relativelocation) (.z _relativelocation)) false false)
    (Transformation|SetRelativeLocation _downtrace_0 (Math|Vector|MakeVector (- (.x _relativelocation_2) 2e+02) (.y _relativelocation_2) (.z _relativelocation_2)) false false)))

(event Input|MouseEvents|MouseWheelUp
  (params (Key :type Key%20Structure :default "None"))
  (bind _playercharacter (Variables|Default|GetPlayerCharacter))
  (bind _begintrace_0 (Variables|/Game/FirstPerson/Blueprints/BP_PlayerCharacter_VortigauntTest.BP_PlayerCharacter_VortigauntTest_C|GetBeginTrace_0 _playercharacter))
  (bind _downtrace_0 (Variables|/Game/FirstPerson/Blueprints/BP_PlayerCharacter_VortigauntTest.BP_PlayerCharacter_VortigauntTest_C|GetDownTrace_0 _playercharacter))
  (bind _relativelocation (Variables|/Script/Engine.SceneComponent|GetRelativeLocation _downtrace_0))
  (bind _relativelocation_2 (Variables|/Script/Engine.SceneComponent|GetRelativeLocation _begintrace_0))
  ;[0.15 0.1159 0.000808 0.5] Mouse Wheele Distance Teleport Modifier
  (:Pressed
    (Transformation|SetRelativeLocation _begintrace_0 (Math|Vector|MakeVector (+ (.x _relativelocation_2) 2e+02) (.y _relativelocation_2) (.z _relativelocation_2)) false false)
    (Transformation|SetRelativeLocation _downtrace_0 (Math|Vector|MakeVector (+ (.x _relativelocation) 2e+02) (.y _relativelocation) (.z _relativelocation)) false false)))

(fn GetTeleportPointsLocations
  (bind _playercharacter (Variables|Default|GetPlayerCharacter))
  (return (Transformation|GetWorldLocation (Variables|/Game/FirstPerson/Blueprints/BP_PlayerCharacter_VortigauntTest.BP_PlayerCharacter_VortigauntTest_C|GetCube_0 _playercharacter)) (Transformation|GetWorldLocation (Variables|/Game/FirstPerson/Blueprints/BP_PlayerCharacter_VortigauntTest.BP_PlayerCharacter_VortigauntTest_C|GetBeginTrace_0 _playercharacter))))

(fn SetTeleportFXLocation
  (params (NewLocation :type Vector))
  (Transformation|SetWorldLocation (Variables|/Game/FirstPerson/Blueprints/BP_PlayerCharacter_VortigauntTest.BP_PlayerCharacter_VortigauntTest_C|GetTeleportTargetPosition_0 (Variables|Default|GetPlayerCharacter)) NewLocation false false))