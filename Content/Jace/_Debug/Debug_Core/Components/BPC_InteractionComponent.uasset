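; Interaction component that lets the player interact with the actor the first-person camera is looking at.
; BeginPlay caches the player character, and OnInteract, gated by its CanInteract flag, line-traces within a maximum distance using the BPI_Interactable interface, with debug drawing.
; A successful trace triggers CallInteraction.
; FindStartAndEndPoint computes camera-forward trace points, but OnInteract uses FindCameraTracePoints instead.
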(event Custom|OnInteract
  (bind _maxinteractiondistance (Variables|Default|GetMaxInteractionDistance))
  (bind (_startpoint _endpoint) (CallFunction|FindCameraTracePoints _maxinteractiondistance))
  (if (Variables|/Game/FirstPerson/Blueprints/BP_PlayerCharacter.BP_PlayerCharacter_C|GetbCanInteract (Variables|Default|GetPlayerCharacter))
    (bind _returnvalue (CallFunction|LineTraceHitActor "ForOneFrame" _startpoint _endpoint "/Game/Jace/_Debug/Debug_Core/Interfaces/BPI_Interactable.BPI_Interactable_C"))
    (if _returnvalue
      (Default|CallInteraction))))

(event EventBeginPlay
  (bind _asbp_player_character (Utilities|Casting|CastToBP_PlayerCharacter (Game|GetPlayerCharacter 0)))
  (Variables|Default|SetPlayerCharacter _asbp_player_character))

(fn FindStartandEndPoint
  (bind _playercharacter (Variables|Default|GetPlayerCharacter))
  (bind _firstpersoncamera (Variables|/Game/FirstPerson/Blueprints/BP_FirstPersonCharacter.BP_FirstPersonCharacter_C|GetFirstPersonCamera _playercharacter))
  (bind _returnvalue (Transformation|GetWorldLocation _firstpersoncamera))
  (return _returnvalue (+ _returnvalue (* (Math|Vector|GetForwardVector (Transformation|GetWorldRotation _firstpersoncamera)) (Variables|Default|GetMaxInteractionDistance)))))