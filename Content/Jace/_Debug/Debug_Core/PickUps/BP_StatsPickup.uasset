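; Physics-simulated stat pickup that raises a configurable player attribute when its trigger is entered.
; It extends a parent pickup's trigger event, reading and writing the attribute through the player character's BPCAttributesComponent.
; If the value is below 100, it adds IncreaseValue without clamping the result, then destroys itself after a short delay; otherwise the pickup remains.
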(event EventTick
  (params (DeltaSeconds :type Float%20%28single-precision%29)))

(event EventBeginPlay
  (|CallParentFunction)
  (Physics|SetSimulatePhysics (Variables|Default|GetStaticMesh) true))

(event EventOnEnterTrigger
  (|CallParentFunction)
  (bind _current_value (CallFunction|GetPlayerAttribute (Variables|Default|GetAttribute)))
  (if (< _current_value 1e+02)
    (CallFunction|IncreasePlayerAttribute)
    (Utilities|FlowControl|Delay 0.2)
    (Actor|DestroyActor)))

(fn ConstructionScript
  (|CallParentFunction))

(fn GetPlayerAttribute
  (params (AttributeName :type Name))
  (return (Default|GetAttributeValue (Variables|/Game/FirstPerson/Blueprints/BP_PlayerCharacter.BP_PlayerCharacter_C|GetBPC_AttributesComponent (Variables|Default|GetPlayerCharacter)) AttributeName)))

(fn IncreasePlayerAttribute
  (bind _attribute (Variables|Default|GetAttribute))
  (bind _current_value (CallFunction|GetPlayerAttribute _attribute))
  (Default|SetAttribute (Variables|/Game/FirstPerson/Blueprints/BP_PlayerCharacter.BP_PlayerCharacter_C|GetBPC_AttributesComponent (Variables|Default|GetPlayerCharacter)) (+ _current_value (Variables|Default|GetIncreaseValue)) _attribute))