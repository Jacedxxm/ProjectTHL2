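; BP_Ammo is a pickup in a debug folder that refills the player's rifle ammo from a random amount rolled between min and max on BeginPlay.
; On trigger entry it plays a sound and adds to the Rebel character's inventory, capped at max rifle ammo.
; Leftover ammo stays in the pickup, which destroys itself once empty.
; Tick prints the remaining amount on screen as debug output.
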(event EventBeginPlay
  (|CallParentFunction)
  (Variables|Default|SetPickupAmmo (Math|Random|RandomIntegerinRange (Variables|Default|GetMinAmmo) (Variables|Default|GetMaxAmmo))))

(event EventTick
  (params (DeltaSeconds :type Float%20%28single-precision%29))
  (|CallParentFunction DeltaSeconds)
  (Development|PrintString (Utilities|String|ToString(Integer) (Variables|Default|GetPickupAmmo)) true true "(R=1.000000,G=0.000000,B=0.906680,A=1.000000)" 0.0))

(event EventOnEnterTrigger
  (|CallParentFunction)
  (if (> (Variables|Default|GetPickupAmmo) 0)
    (Audio|PlaySound2D "/Game/ThirdParty/MilitaryWeapSilver/Sound/Pistol/Wavs/Pistol_AmmoPickup.Pistol_AmmoPickup" 1.0 1.0 0.0 0 0)
    (bind _asbp_player_character_rebel (Utilities|Casting|CastToBP_PlayerCharacter_Rebel (Variables|Default|GetPlayerCharacter)))
    (bind _output_get (Variables|Default|SetPlayerInventory (Variables|/Game/FirstPerson/Blueprints/BP_PlayerCharacter_Rebel.BP_PlayerCharacter_Rebel_C|GetBP_PlayerInventory _asbp_player_character_rebel)))
    (Variables|Default|SetAmmoToAdd (Math|Integer|Min(Integer) (- (Variables|/Game/Jace/_Debug/Debug_Core/Components/BP_PlayerInventory.BP_PlayerInventory_C|GetMaxRifleAmmo _output_get) (Variables|/Game/Jace/_Debug/Debug_Core/Components/BP_PlayerInventory.BP_PlayerInventory_C|GetCurrentRifleAmmo _output_get)) (Variables|Default|GetPickupAmmo)))
    (Variables|/Game/Jace/_Debug/Debug_Core/Components/BP_PlayerInventory.BP_PlayerInventory_C|SetCurrentRifleAmmo (Variables|Default|GetPlayerInventory) (+ (Variables|/Game/Jace/_Debug/Debug_Core/Components/BP_PlayerInventory.BP_PlayerInventory_C|GetCurrentRifleAmmo (Variables|Default|GetPlayerInventory)) (Variables|Default|GetAmmoToAdd)))
    (bind _output_get_2 (Variables|Default|SetPickupAmmo (- (Variables|Default|GetPickupAmmo) (Variables|Default|GetAmmoToAdd))))
    (if (<= _output_get_2 0)
      (Actor|DestroyActor))
    (else
      (Utilities|FlowControl|Delay 0.2)
      (Actor|DestroyActor))))

(fn ConstructionScript
  (|CallParentFunction))