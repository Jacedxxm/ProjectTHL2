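; BP_StatsPickupable is a pickup Blueprint in the debug core folder that raises one of the player's attributes.
; On trigger entry it runs the parent handler, then reads the player attribute selected by its Attribute variable.
; If that value is below 100, it increases the attribute and destroys itself after a short delay; otherwise it stays in the world.
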(event EventBeginPlay
  (|CallParentFunction) ; This node is disabled and will not be called.\nDrag off pins to build functionality.
)

(event EventTick
  (params (DeltaSeconds :type Float%20%28single-precision%29))
  (|CallParentFunction DeltaSeconds) ; This node is disabled and will not be called.\nDrag off pins to build functionality.
)

(event EventOnEnterTrigger
  (|CallParentFunction)
  (bind _current_value (CallFunction|GetPlayerAttribute (Variables|Default|GetAttribute)))
  (if (< _current_value 1e+02)
    (CallFunction|IncreasePlayerAttribute)
    (Utilities|FlowControl|Delay 0.2)
    (Actor|DestroyActor)))

(fn ConstructionScript
  (|CallParentFunction))