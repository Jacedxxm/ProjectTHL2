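; BP_CargoShip is a cargo ship actor that drops vertically when its linked computer is activated.
; On BeginPlay it binds DropShip to the PC activation event on ComputerRef and stores its starting location.
; DropShip plays a cargo drop sound, then a timeline lerps the actor straight down from that location by a fixed distance, without sweeping for collision.
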(event Custom|DropShip
  (bind _startinglocation (Variables|Default|GetStartingLocation))
  (Audio|PlaySoundatLocation "/Game/Jace/_Debug/Debug_Core/Audio/Cargoship/SC_CargoDrop.SC_CargoDrop" (Transformation|GetActorLocation) "0, 0, 0" 1.0 1.0 0.0 0 0 0 0)
  (bind _alpha (Timeline|CargoShipAnimation PlayFromStart)
    (:Update
      (Transformation|SetActorLocation (Math|Vector|Lerp(Vector) (Math|Vector|MakeVector (.x _startinglocation) (.y _startinglocation) (.z _startinglocation)) (Math|Vector|MakeVector (.x _startinglocation) (.y _startinglocation) (- (.z _startinglocation) 2.5e+03)) _alpha) false false))))

(event EventBeginPlay
  (EventDispatchers|BindEventtoOnPcActivation (Variables|Default|GetComputerRef) (delegate Custom|DropShip))
  (Variables|Default|SetStartingLocation (Transformation|GetActorLocation)))

(fn ConstructionScript)