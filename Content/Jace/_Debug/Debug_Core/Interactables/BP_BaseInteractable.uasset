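; BP_BaseInteractable is a debug-folder base Blueprint for objects the player can interact with when nearby.
; A sphere trigger sets CanBeInteracted when the player character enters and clears it on exit.
; The Interaction event checks that flag and, when true, plays InteractionSound at the actor's location.
; BeginPlay caches a reference to the player character.
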(event OnComponentBeginOverlap(Sphere)
  (params (OverlappedComponent :type Primitive%20Component%20Object%20Reference) (OtherActor :type Actor%20Object%20Reference) (OtherComp :type Primitive%20Component%20Object%20Reference) (OtherBodyIndex :type Integer) (bFromSweep :type Boolean) (SweepResult :type Hit%20Result%20Structure%20%28by%20ref%29))
  (Utilities|CheckforPlayerCharacter OtherActor
    (:true
      (Variables|Default|SetbCanBeInteracted true))))

(event OnComponentEndOverlap(Sphere)
  (params (OverlappedComponent :type Primitive%20Component%20Object%20Reference) (OtherActor :type Actor%20Object%20Reference) (OtherComp :type Primitive%20Component%20Object%20Reference) (OtherBodyIndex :type Integer))
  (Utilities|CheckforPlayerCharacter OtherActor
    (:true
      (Variables|Default|SetbCanBeInteracted false))))

(event EventBeginPlay
  (bind _playerref (CallFunction|GetPlayerReference))
  (Variables|Default|SetPlayerCharacter _playerref))

(event EventInteraction
  (if (Variables|Default|GetbCanBeInteracted)
    (Audio|PlaySoundatLocation (Variables|Default|GetInteractionSound) (Transformation|GetActorLocation) "0, 0, 0" 1.0 1.0 0.0 0 0 0 0)))

(fn ConstructionScript)