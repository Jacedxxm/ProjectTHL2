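; BP_GateLever is an interactable lever that becomes usable once a referenced tank is activated.
; At BeginPlay it binds to the player's interaction component and to the tank's OnTankActivated event, with tank activation marking the lever available.
; When activated while available and interactable, it calls Activate, broadcasts OnLeverActivated and clears both flags, locking itself after use.
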(event Custom|OnTankActivation
  (Variables|Default|SetbIsAvailable true))

(event Custom|ActivateLever
  (|CallParentFunction)
  (if (and (Variables|Default|GetbIsAvailable) (Variables|Default|GetbCanBeInteracted))
    (CallFunction|Activate)
    (Default|CallOnLeverActivated)
    (Variables|Default|SetbIsAvailable false)
    (Variables|Default|SetbCanBeInteracted false)))

(event EventBeginPlay
  (|CallParentFunction)
  (EventDispatchers|BindEventtoInteraction (Variables|/Game/FirstPerson/Blueprints/BP_PlayerCharacter.BP_PlayerCharacter_C|GetBPC_InteractionComponent (Variables|Default|GetPlayerCharacter)) (EventDispatchers|CreateEvent :!event Custom|ActivateLever))
  (EventDispatchers|BindEventtoOnTankActivated (Variables|Default|GetTankRef) (EventDispatchers|CreateEvent :!event Custom|OnTankActivation)))

(event EventInteraction
  (|CallParentFunction))

(fn ConstructionScript
  (|CallParentFunction))