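; BP_TowerLever is a one-shot interactable lever, apparently for a tower, that notifies listeners when pulled.
; On BeginPlay it binds its activation event to the player character's interaction component.
; When an interaction fires while the lever is interactable and available, it calls Activate, broadcasts OnTowerLeverActivated, then marks itself activated and unavailable.
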(event Custom|ActivarteLever
  (if (and (Variables|Default|GetbCanBeInteracted) (Variables|Default|GetbIsAvailable))
    (CallFunction|Activate)
    (Default|CallOnTowerLeverActivated)
    (Variables|Default|SetbIsAvailable false)
    (Variables|Default|SetbActivated true)))

(event EventBeginPlay
  (|CallParentFunction)
  (EventDispatchers|BindEventtoInteraction (Variables|/Game/FirstPerson/Blueprints/BP_PlayerCharacter.BP_PlayerCharacter_C|GetBPC_InteractionComponent (Variables|Default|GetPlayerCharacter)) (delegate Custom|ActivarteLever)))

(fn ConstructionScript
  (|CallParentFunction))