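; BP_BaseLever is a base lever interactable that swings its mesh between a closed and an open rotation.
; At BeginPlay it snaps the mesh to the closed rotation.
; Activate plays a timeline that lerps only the pitch from closed to open, keeping closed roll and yaw, and Deactivate reverses that timeline from the end.
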(event Custom|Activate
  (bind _closedrotation (Variables|Default|GetClosedRotation))
  (bind _newtrack_0 (Timeline|ActivateAnimation Play)
    (:Update
      (Transformation|SetRelativeRotation (Variables|Default|GetStaticMesh_0) (Math|Rotator|MakeRotator (.roll _closedrotation) (Math|Float|Lerp (.pitch _closedrotation) (.pitch (Variables|Default|GetOpenRotation)) _newtrack_0) (.yaw _closedrotation)) false false))))

(event Custom|Deactivate
  (bind _closedrotation (Variables|Default|GetClosedRotation))
  (bind _newtrack_0 (Timeline|ActivateAnimation ReverseFromEnd)
    (:Update
      (Transformation|SetRelativeRotation (Variables|Default|GetStaticMesh_0) (Math|Rotator|MakeRotator (.roll _closedrotation) (Math|Float|Lerp (.pitch _closedrotation) (.pitch (Variables|Default|GetOpenRotation)) _newtrack_0) (.yaw _closedrotation)) false false))))

(event EventBeginPlay
  (|CallParentFunction)
  (Transformation|SetRelativeRotation (Variables|Default|GetStaticMesh_0) (Variables|Default|GetClosedRotation) false false))

(fn ConstructionScript)