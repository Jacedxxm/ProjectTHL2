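; Debug Vortigaunt dialogue trigger that plays a timed, voiced conversation when the player walks into its sphere.
; On overlap, if interaction is allowed, it casts to the Vortigaunt test character and shows the dialogue text on that player's attributes HUD.
; Delays sequence two sound-backed lines, then send a final line through a separate PlayerCharacter reference and immediately hide the text.
; CanBeInteracted is only read here, never cleared.
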(event OnComponentBeginOverlap(Sphere)
  (params (OverlappedComponent :type Primitive%20Component%20Object%20Reference) (OtherActor :type Actor%20Object%20Reference) (OtherComp :type Primitive%20Component%20Object%20Reference) (OtherBodyIndex :type Integer) (bFromSweep :type Boolean) (SweepResult :type Hit%20Result%20Structure%20%28by%20ref%29))
  (bind _playercharacter (Variables|Default|GetPlayerCharacter))
  (bind _playerattributeshud (Variables|/Game/FirstPerson/Blueprints/BP_PlayerCharacter.BP_PlayerCharacter_C|GetPlayerAttributesHUD _playercharacter))
  (if (and (== OtherActor (Game|GetPlayerCharacter 0)) (Variables|Default|GetbCanBeInteracted))
    (bind _asbp_player_character_vortigaunt_test (Utilities|Casting|CastToBP_PlayerCharacter_VortigauntTest (Game|GetPlayerCharacter 0)))
    (Variables|/Script/UMG.Widget|SetVisibility (Variables|/Game/Jace/_Debug/Debug_Core/UserInterface/WBP_HUD.WBP_HUD_C|GetDialogueText (Variables|/Game/FirstPerson/Blueprints/BP_PlayerCharacter.BP_PlayerCharacter_C|GetPlayerAttributesHUD _asbp_player_character_vortigaunt_test)) "Visible")
    (Audio|PlaySoundatLocation (Variables|Default|GetDialogueSound) (Transformation|GetActorLocation) "0, 0, 0" 1.0 1.0 0.0 0 0 0 0)
    (Default|TriggerDialogue (Variables|/Game/FirstPerson/Blueprints/BP_PlayerCharacter.BP_PlayerCharacter_C|GetPlayerAttributesHUD _asbp_player_character_vortigaunt_test) (Variables|Default|GetFirstDialogue))
    (Utilities|FlowControl|Delay (Variables|Default|GetTimeBeforeSecondDialogue))
    (Audio|PlaySoundatLocation (Variables|Default|GetDialogueSound2) (Transformation|GetActorLocation) "0, 0, 0" 1.0 1.0 0.0 0 0 0 0)
    (Default|TriggerDialogue (Variables|/Game/FirstPerson/Blueprints/BP_PlayerCharacter.BP_PlayerCharacter_C|GetPlayerAttributesHUD _asbp_player_character_vortigaunt_test) (Variables|Default|GetSecondDialogue))
    (Utilities|FlowControl|Delay (Variables|Default|GetTimeToFinishLastDialogue))
    (Default|TriggerDialogue _playerattributeshud (Variables|Default|GetFinalDialogue))
    (Variables|/Script/UMG.Widget|SetVisibility (Variables|/Game/Jace/_Debug/Debug_Core/UserInterface/WBP_HUD.WBP_HUD_C|GetDialogueText _playerattributeshud) "Hidden")))

(event EventBeginPlay
  (|CallParentFunction))

(fn ConstructionScript
  (|CallParentFunction))