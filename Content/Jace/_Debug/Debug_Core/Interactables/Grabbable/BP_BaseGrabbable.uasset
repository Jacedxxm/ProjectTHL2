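; Base Blueprint for grabbable physics objects in a debug interactables set, handling how the object is thrown.
; The ThrowObject event passes its force to AddPhysicImpulse, which launches the static mesh along the forward vector of player 0's camera.
; It emulates an impulse by setting linear velocity to force divided by mass, replacing any current velocity, so heavier objects fly slower.
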(event EventThrowObject
  (params (ImpulseForce :type Float%20%28double-precision%29))
  (CallFunction|AddPhysicImpulse ImpulseForce))

(fn ConstructionScript)

(fn AddPhysicImpulse
  (params (ImpulseForce :type Float%20%28single-precision%29))
  (Physics|SetPhysicsLinearVelocity (Variables|Default|GetStaticMesh) (/ (* (Math|Vector|GetForwardVector (Camera|GetCameraRotation (Variables|/Script/Engine.PlayerController|GetPlayerCameraManager (Game|GetPlayerController 0)))) ImpulseForce) (Physics|GetMass (Variables|Default|GetStaticMesh))) false "None"))