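; Interactable note actor that shows a readable title and description in a WBP_Note widget.
; It creates the widget on BeginPlay and binds an event to the player's interaction component on overlap.
; Interaction fills and displays the widget only while IsReading is false, then sets that flag.
; Ending overlap removes the widget but leaves IsReading set, so this graph does not reopen it.
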(event EventBeginPlay
  (|CallParentFunction)
  (bind _returnvalue (UserInterface|CreateWidget "/Game/Jace/_Debug/Debug_Core/UserInterface/WBP_Note.WBP_Note_C" (Game|GetPlayerController 0)))
  (Variables|Default|SetNoteWidget _returnvalue)
  (Variables|Default|SetbIsReading false))

(event Collision|EventActorBeginOverlap
  (params (OtherActor :type Actor%20Object%20Reference))
  (|CallParentFunction OtherActor)
  (EventDispatchers|BindEventtoInteraction (Variables|/Game/FirstPerson/Blueprints/BP_PlayerCharacter.BP_PlayerCharacter_C|GetBPC_InteractionComponent (Variables|Default|GetPlayerCharacter)) (EventDispatchers|CreateEvent :!event Interaction)))

(event Collision|EventActorEndOverlap
  (params (OtherActor :type Actor%20Object%20Reference))
  (|CallParentFunction OtherActor)
  (Widget|RemovefromParent (Variables|Default|GetNoteWidget)))

(event EventInteraction
  (|CallParentFunction)
  (if (not (Variables|Default|GetbIsReading))
    (Variables|Default|SetbIsReading true)
    (bind _aswbp_note (Utilities|Casting|CastToWBP_Note (Variables|Default|GetNoteWidget)))
    (Default|Open _aswbp_note (Variables|Default|GetNoteTitle) (Variables|Default|GetNoteDescription))
    (UserInterface|Viewport|AddtoViewport (Variables|Default|GetNoteWidget) 0)))

(fn ConstructionScript
  (|CallParentFunction))