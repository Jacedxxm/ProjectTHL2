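; Interactable Vortigaunt Blueprint that plays a timed, three-line dialogue on the player's HUD.
; BeginPlay binds an event to the player's interaction component, and StartingDialogue runs the sequence if CanBeInteracted is true.
; Delays space the lines, with a sound at the actor's location for the first two.
; The HUD text is hidden immediately after the final line triggers, with no delay between.
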(event Custom|StartingDialogue
  (bind _playercharacter (Variables|Default|GetPlayerCharacter))
  (bind _playercharacter_2 (Variables|Default|GetPlayerCharacter))
  (bind _playerattributeshud (Variables|/Game/FirstPerson/Blueprints/BP_PlayerCharacter.BP_PlayerCharacter_C|GetPlayerAttributesHUD _playercharacter))
  (bind _playerattributeshud_2 (Variables|/Game/FirstPerson/Blueprints/BP_PlayerCharacter.BP_PlayerCharacter_C|GetPlayerAttributesHUD _playercharacter_2))
  (if (Variables|Default|GetbCanBeInteracted)
    (Variables|/Script/UMG.Widget|SetVisibility (Variables|/Game/Jace/_Debug/Debug_Core/UserInterface/WBP_HUD.WBP_HUD_C|GetDialogueText _playerattributeshud_2) "Visible")
    (Audio|PlaySoundatLocation (Variables|Default|GetDialogueSound) (Transformation|GetActorLocation) "0, 0, 0" 1.0 1.0 0.0 0 0 0 0)
    (Default|TriggerDialogue _playerattributeshud_2 (Variables|Default|GetFirstDialogue))
    (Utilities|FlowControl|Delay 3.0)
    (Audio|PlaySoundatLocation (Variables|Default|GetDialogueSound) (Transformation|GetActorLocation) "0, 0, 0" 1.0 1.0 0.0 0 0 0 0)
    (Default|TriggerDialogue (Variables|/Game/FirstPerson/Blueprints/BP_PlayerCharacter.BP_PlayerCharacter_C|GetPlayerAttributesHUD (Variables|Default|GetPlayerCharacter)) (Variables|Default|GetSecondDialogue))
    (Utilities|FlowControl|Delay 4.0)
    (Default|TriggerDialogue _playerattributeshud (Variables|Default|GetFinalDialogue))
    (Variables|/Script/UMG.Widget|SetVisibility (Variables|/Game/Jace/_Debug/Debug_Core/UserInterface/WBP_HUD.WBP_HUD_C|GetDialogueText _playerattributeshud) "Hidden")))

(event EventBeginPlay
  (|CallParentFunction)
  (EventDispatchers|BindEventtoInteraction (Variables|/Game/FirstPerson/Blueprints/BP_PlayerCharacter.BP_PlayerCharacter_C|GetBPC_InteractionComponent (Variables|Default|GetPlayerCharacter)) (EventDispatchers|CreateEvent :!event Custom|StartingDialogue)))

(fn ConstructionScript
  (|CallParentFunction))