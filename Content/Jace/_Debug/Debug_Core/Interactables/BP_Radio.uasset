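; BP_Radio is an interactable radio that calls in a helicopter once the referenced tower lever is activated.
; It binds to the player's interaction component and, when interaction is allowed, plays an off sound if the lever is inactive.
; Otherwise a delay-timed sequence shows HUD dialogue, then reveals and triggers the helicopter with its audio.
; After a further helicopter sound, it fires OnRadioTriggered.
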(event Custom|RadioInteraction
  (bind _playercharacter (Variables|Default|GetPlayerCharacter))
  (bind _playerattributeshud (Variables|/Game/FirstPerson/Blueprints/BP_PlayerCharacter.BP_PlayerCharacter_C|GetPlayerAttributesHUD _playercharacter))
  (Audio|PlaySound2D "/Game/Jace/_Debug/Debug_Core/Audio/Radio/SC_RadioHL.SC_RadioHL" 1.0 1.0 0.0 0 0)
  (Default|TriggerDialogue _playerattributeshud "...")
  (Variables|/Script/UMG.Widget|SetVisibility (Variables|/Game/Jace/_Debug/Debug_Core/UserInterface/WBP_HUD.WBP_HUD_C|GetDialogueText _playerattributeshud) "Visible")
  (Utilities|FlowControl|Delay 2.0)
  (Default|TriggerDialogue _playerattributeshud "...")
  (Utilities|FlowControl|Delay 2.0)
  (Variables|/Script/UMG.Widget|SetVisibility (Variables|/Game/Jace/_Debug/Debug_Core/UserInterface/WBP_HUD.WBP_HUD_C|GetDialogueText _playerattributeshud) "Hidden")
  (CallFunction|SetHelicopterActive)
  (Utilities|FlowControl|Delay 6.0)
  (Audio|PlaySound2D "/Game/Jace/_Debug/Debug_Core/Audio/SC_HelicopterSoundHL.SC_HelicopterSoundHL" 1.0 1.0 0.0 0 0)
  (Utilities|FlowControl|Delay 3.0)
  (Default|CallOnRadioTriggered))

(event EventBeginPlay
  (|CallParentFunction)
  (EventDispatchers|BindEventtoInteraction (Variables|/Game/FirstPerson/Blueprints/BP_PlayerCharacter.BP_PlayerCharacter_C|GetBPC_InteractionComponent (Variables|Default|GetPlayerCharacter)) (EventDispatchers|CreateEvent :!event Interaction))
  (Variables|Default|SetbSecondInteraction false))

(event EventInteraction
  (|CallParentFunction)
  (if (Variables|Default|GetbCanBeInteracted)
    (if (Variables|/Game/Jace/_Debug/Debug_Core/Interactables/Lever/BP_TowerLever.BP_TowerLever_C|GetbActivated (Variables|Default|GetTowerLeverRef))
      (CallFunction|RadioInteraction)
      (else
        (Audio|PlaySound2D "/Game/Jace/_Debug/Debug_Core/Audio/Radio/SC_RadioHLOFf.SC_RadioHLOFf" 1.0 1.0 0.0 0 0)))))

(fn ConstructionScript
  (|CallParentFunction))

(fn SetHelicopterActive
  (bind _helicopter (Variables|Default|GetHelicopter))
  (Rendering|SetVisibility (Variables|/Game/ThirdParty/Sci_FI_Valley_Village/BP/Ship_flying/BP_FlyingMesh.BP_FlyingMesh_C|GetSM_ship _helicopter) true false)
  (Rendering|SetVisibility (Variables|/Game/ThirdParty/Sci_FI_Valley_Village/BP/Ship_flying/BP_FlyingMesh.BP_FlyingMesh_C|GetRotor _helicopter) true false)
  (Variables|/Game/ThirdParty/Sci_FI_Valley_Village/BP/Ship_flying/BP_FlyingMesh.BP_FlyingMesh_C|SetbIsTriggered _helicopter true)
  (Components|Activation|Activate (Variables|/Game/ThirdParty/Sci_FI_Valley_Village/BP/Ship_flying/BP_FlyingMesh.BP_FlyingMesh_C|GetAudio _helicopter) false))