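; Debug fluid tank interactable that activates when a grabbable cable is plugged into it.
; The first cable to overlap the box snaps to the connector, loses physics and collision, and is released from the player's grab component, with sparks and sound.
; It then calls the OnTankActivated dispatcher and runs a timeline that scales the liquid mesh vertically from its starting height to show the fluid level changing.
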(event OnComponentBeginOverlap(Box)
  (params (OverlappedComponent :type Primitive%20Component%20Object%20Reference) (OtherActor :type Actor%20Object%20Reference) (OtherComp :type Primitive%20Component%20Object%20Reference) (OtherBodyIndex :type Integer) (bFromSweep :type Boolean) (SweepResult :type Hit%20Result%20Structure%20%28by%20ref%29))
  (bind _asbp_grabbable_cable (Utilities|Casting|CastToBP_GrabbableCable OtherActor))
  (Utilities|FlowControl|DoOnce false
    (:Completed
      (Transformation|SetWorldTransform (Variables|/Game/Jace/_Debug/Debug_Core/Interactables/Cable/BP_GrabbableCable.BP_GrabbableCable_C|GetCube _asbp_grabbable_cable) (Transformation|GetWorldTransform (Variables|Default|GetConnector)) false false)
      (Physics|SetSimulatePhysics (Variables|/Game/Jace/_Debug/Debug_Core/Interactables/Cable/BP_GrabbableCable.BP_GrabbableCable_C|GetCube _asbp_grabbable_cable) false)
      (Variables|/Game/Jace/_Debug/Debug_Core/Components/BPC_GrabComponent.BPC_GrabComponent_C|SetbIsGrabbingObject (Variables|/Game/FirstPerson/Blueprints/BP_PlayerCharacter.BP_PlayerCharacter_C|GetBPC_GrabComponent (Variables|Default|GetPlayerCharacter)) false)
      (Audio|PlaySoundatLocation "/Game/Jace/_Debug/Debug_Core/Audio/SC_Cable.SC_Cable" (.location (Transformation|GetWorldTransform (Variables|Default|GetConnector))) "0, 0, 0" 1.0 1.0 0.0 0 0 0 0)
      (Effects|SpawnEmitteratLocation "/Game/StarterContent/Particles/P_Sparks.P_Sparks" (Transformation|GetWorldLocation (Variables|/Game/Jace/_Debug/Debug_Core/Interactables/Cable/BP_GrabbableCable.BP_GrabbableCable_C|GetCube _asbp_grabbable_cable)))
      (Collision|SetActorEnableCollision _asbp_grabbable_cable false)
      (Default|CallOnTankActivated)
      (CallFunction|ActivateTank))))

(event Custom|ActivateTank
  (bind _startliquidscale (Variables|Default|GetStartLiquidScale))
  (Audio|PlaySoundatLocation "/Game/StarterContent/Audio/Smoke01.Smoke01" (Transformation|GetActorLocation) "0, 0, 0" 1.0 1.0 0.0 0 0 0 0)
  (bind _alpha (Timeline|FluidAnimation Play)
    (:Update
      (Transformation|SetWorldScale3D (Variables|Default|GetSM_TankLiquid) (Math|Vector|MakeVector (.x _startliquidscale) (.y _startliquidscale) (Math|Float|Lerp (.z _startliquidscale) 7.5 _alpha))))))

(event EventBeginPlay
  (bind _playerref (CallFunction|GetPlayerReference))
  (Variables|Default|SetPlayerCharacter _playerref)
  (Variables|Default|SetStartLiquidScale (Variables|/Script/Engine.SceneComponent|GetRelativeScale3D (Variables|Default|GetSM_TankLiquid))))

(fn ConstructionScript)