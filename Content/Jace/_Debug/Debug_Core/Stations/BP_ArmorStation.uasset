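; Armor recharge station, a child of a base station class, that restores the player's Armor attribute from a limited capacity.
; Overlap and interaction defer to the parent, while Heal/Recharge transfers a frame-time-scaled amount, clamped to remaining capacity, through the player's attributes component.
; A TextRender displays the remaining capacity, and recharging stops when Armor reaches a hard-coded 100 or capacity runs out.
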(event EventBeginPlay
  (|CallParentFunction)
  (Rendering|Components|TextRender|SetText (Variables|Default|GetTextRender) (Utilities|Text|ToText(Float) (Variables|Default|GetCurrentCapacity) "HalfToEven")))

(event Collision|EventActorBeginOverlap
  (params (OtherActor :type Actor%20Object%20Reference))
  (|CallParentFunction OtherActor))

(event Collision|EventActorEndOverlap
  (params (OtherActor :type Actor%20Object%20Reference))
  (|CallParentFunction OtherActor))

(event EventInteraction
  (|CallParentFunction))

(event EventHeal/Recharge
  (bind _returnvalue (Utilities|Time|GetWorldDeltaSeconds))
  (bind _recoveryperseconds (Variables|Default|GetRecoveryPerSeconds))
  (bind _returnvalue_2 (* _recoveryperseconds _returnvalue))
  (|CallParentFunction)
  (if (== (Default|GetAttributeValue (Variables|/Game/FirstPerson/Blueprints/BP_PlayerCharacter.BP_PlayerCharacter_C|GetBPC_AttributesComponent (Variables|Default|GetPlayerCharacter)) "Armor") 1e+02)
    (CallFunction|StopHealing/Recharging)
    (elif (> (Variables|Default|GetCurrentCapacity) 0.0)
      (bind _output_get (Variables|Default|SetAmountToHeal _returnvalue_2))
      (bind _output_get_2 (Variables|Default|SetAmountToHeal (Math|Float|Min(Float) _output_get (Variables|Default|GetCurrentCapacity) _returnvalue_2)))
      (bind _output_get_3 (Variables|Default|SetCurrentCapacity (- (Variables|Default|GetCurrentCapacity) _output_get_2)))
      (if (and (> _output_get_3 0.0) (< (Default|GetAttributeValue (Variables|/Game/FirstPerson/Blueprints/BP_PlayerCharacter.BP_PlayerCharacter_C|GetBPC_AttributesComponent (Variables|Default|GetPlayerCharacter)) "Armor") (Variables|Default|GetPlayerMaxArmor)))
        (Default|SetAttribute (Variables|/Game/FirstPerson/Blueprints/BP_PlayerCharacter.BP_PlayerCharacter_C|GetBPC_AttributesComponent (Variables|Default|GetPlayerCharacter)) (Math|Float|Lerp (Default|GetAttributeValue (Variables|/Game/FirstPerson/Blueprints/BP_PlayerCharacter.BP_PlayerCharacter_C|GetBPC_AttributesComponent (Variables|Default|GetPlayerCharacter)) "Armor") (+ (Variables|Default|GetAmountToHeal) (Default|GetAttributeValue (Variables|/Game/FirstPerson/Blueprints/BP_PlayerCharacter.BP_PlayerCharacter_C|GetBPC_AttributesComponent (Variables|Default|GetPlayerCharacter)) "Armor")) 1.0) "Armor")
        (bind _valuetext (CallFunction|TruncateValuetoText (Variables|Default|GetCurrentCapacity)))
        (Rendering|Components|TextRender|SetText (Variables|Default|GetTextRender) _valuetext))
      (else
        (CallFunction|StopHealing/Recharging)))))

(event EventStopHealing/Recharging
  (|CallParentFunction))

(fn ConstructionScript
  (|CallParentFunction))

(fn SetAmounttoHeal
  (params (Value :type Float%20%28double-precision%29))
  (return false))