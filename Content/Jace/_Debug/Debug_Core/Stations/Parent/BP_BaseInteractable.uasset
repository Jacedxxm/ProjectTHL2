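; Debug parent Blueprint for interactable stations that run a heal/recharge action while the player holds E.
; A sphere overlap filtered to the player toggles CanInteract and actor tick.
; The player's interaction component event copies that into CanHeal, which lets Tick poll E and call the heal or stop events.
; These events only print debug text and play start/stop sounds through two mutually resetting DoOnce gates.
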(event OnComponentBeginOverlap(Sphere)
  (params (OverlappedComponent :type Primitive%20Component%20Object%20Reference) (OtherActor :type Actor%20Object%20Reference) (OtherComp :type Primitive%20Component%20Object%20Reference) (OtherBodyIndex :type Integer) (bFromSweep :type Boolean) (SweepResult :type Hit%20Result%20Structure%20%28by%20ref%29))
  (Utilities|PlayerTrigger OtherActor
    (:True
      (Variables|Default|SetCanInteract true)
      (Actor|Tick|SetActorTickEnabled true))))

(event OnComponentEndOverlap(Sphere)
  (params (OverlappedComponent :type Primitive%20Component%20Object%20Reference) (OtherActor :type Actor%20Object%20Reference) (OtherComp :type Primitive%20Component%20Object%20Reference) (OtherBodyIndex :type Integer))
  (Utilities|PlayerTrigger OtherActor
    (:True
      (Variables|Default|SetCanInteract false)
      (Actor|Tick|SetActorTickEnabled false))))

(event Custom|Heal/Recharge
  (Development|PrintString "Healing")
  (Utilities|FlowControl|DoOnce false
    (:Completed
      (Audio|PlaySound2D "/Engine/VREditor/Sounds/UI/Dockable_Window_Close.Dockable_Window_Close" 1.0 1.0 0.0 0 0)
      (Utilities|FlowControl|DoOnce false) ; enters at Reset
    )))

(event Custom|StopHealing/Recharging
  (Development|PrintString "NotHealing")
  (Utilities|FlowControl|DoOnce false
    (:Completed
      (Audio|PlaySound2D "/Engine/VREditor/Sounds/UI/Dockable_Window_Open.Dockable_Window_Open" 1.0 1.0 0.0 0 0)
      (Utilities|FlowControl|DoOnce false) ; enters at Reset
    )))

(event EventBeginPlay
  (bind _asbp_player_character (Utilities|Casting|CastToBP_PlayerCharacter (Game|GetPlayerCharacter 0)))
  (Variables|Default|SetPlayerCharacter _asbp_player_character)
  (EventDispatchers|BindEventtoInteraction (Variables|/Game/FirstPerson/Blueprints/BP_PlayerCharacter.BP_PlayerCharacter_C|GetBPC_InteractionComponent (Variables|Default|GetPlayerCharacter)) (EventDispatchers|CreateEvent :!event Interaction)))

(event EventInteraction
  (if (Variables|Default|GetCanInteract)
    (Variables|Default|SetbCanHeal true)
    (else
      (Variables|Default|SetbCanHeal false))))

(event EventTick
  (params (DeltaSeconds :type Float%20%28single-precision%29))
  (if (Variables|Default|GetbCanHeal)
    (if (Game|Player|IsInputKeyDown (Game|GetPlayerController 0) "E")
      (Variables|Default|SetbIsInteracting true)
      (CallFunction|Heal/Recharge)
      (else
        (Variables|Default|SetbIsInteracting false)
        (CallFunction|StopHealing/Recharging)))
    (else
      (Development|PrintString "NotHealing"))))

(fn ConstructionScript)