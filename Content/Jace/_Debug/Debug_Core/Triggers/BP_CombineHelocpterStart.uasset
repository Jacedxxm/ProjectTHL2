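; Debug trigger Blueprint that gates its parent trigger behavior, named for starting a Combine helicopter, behind a computer activation.
; On BeginPlay it binds OnCargoDrop to the Computer's OnPcActivation event, which sets a CanBeTriggered flag.
; Entering the trigger calls the parent's OnEnterTrigger logic only when that flag is set, and the flag is never reset here.
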(event Custom|OnCargoDrop
  (Variables|Default|SetbCanBeTriggered true))

(event EventBeginPlay
  (|CallParentFunction)
  (EventDispatchers|BindEventtoOnPcActivation (Variables|Default|GetComputer) (delegate Custom|OnCargoDrop)))

(event EventOnEnterTrigger
  (if (Variables|Default|GetbCanBeTriggered)
    (|CallParentFunction)))

(fn ConstructionScript
  (|CallParentFunction))