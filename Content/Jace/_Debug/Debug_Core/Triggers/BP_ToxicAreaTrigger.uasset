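; Debug trigger volume that deals periodic toxic damage to the player while they are inside it.
; Entering starts a looping timer at DamageTickTime that plays a 2D damage sound and subtracts Damage from the Health attribute on the player's BPCAttributesComponent.
; Exiting clears the timer and resets the IsPlayerInToxicArea flag, building on enter and exit events from a parent trigger class.
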(event Custom|DamagePlayerTimer
  (bind _returnvalue (Utilities|Time|SetTimerbyEvent (delegate Custom|DamagePlayer) (Variables|Default|GetDamageTickTime) true))
  (Variables|Default|SetDamageTimer _returnvalue))

(event Custom|StopDamagePlayer
  (Utilities|Time|ClearandInvalidateTimerbyHandle (Variables|Default|GetDamageTimer)))

(event Custom|DamagePlayer
  (bind _playercharacter (Variables|Default|GetPlayerCharacter))
  (bind _bpc_attributescomponent (Variables|/Game/FirstPerson/Blueprints/BP_PlayerCharacter.BP_PlayerCharacter_C|GetBPC_AttributesComponent _playercharacter))
  (Audio|PlaySound2D "/Game/Jace/_Debug/Debug_Core/Audio/SC_ToxicDamage.SC_ToxicDamage" 1.0 1.0 0.0 0 0)
  (Default|SetAttribute _bpc_attributescomponent (- (Default|GetAttributeValue _bpc_attributescomponent "Health") (Variables|Default|GetDamage)) "Health"))

(event EventBeginPlay
  (|CallParentFunction))

(event EventOnEnterTrigger
  (|CallParentFunction)
  (Variables|Default|SetbIsPlayerInToxicArea true)
  (CallFunction|DamagePlayerTimer))

(event EventOnExitTrigger
  (|CallParentFunction)
  (Variables|Default|SetbIsPlayerInToxicArea false)
  (CallFunction|StopDamagePlayer))

(fn ConstructionScript
  (|CallParentFunction))