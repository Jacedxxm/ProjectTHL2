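; Trigger Blueprint, under the debug core triggers, that shows a tutorial widget when the trigger is entered.
; It extends a parent trigger's enter and exit events; a DoOnce limits display to the first entry, after a configurable delay.
; The configured widget class is created for player 0 and added to the viewport, then removed on exit if valid.
; Exiting does not cancel a pending delay.
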(event EventBeginPlay
  (|CallParentFunction) ; This node is disabled and will not be called.\nDrag off pins to build functionality.
)

(event EventOnEnterTrigger
  (|CallParentFunction)
  (Utilities|FlowControl|DoOnce false
    (:Completed
      (Utilities|FlowControl|Delay (Variables|Default|GetDelay))
      (bind _returnvalue (UserInterface|CreateWidget (Variables|Default|GetTutorialWidget) (Game|GetPlayerController 0)))
      (bind _output_get (Variables|Default|SetTutorialWidgetRef _returnvalue))
      (UserInterface|Viewport|AddtoViewport _output_get 0))))

(event EventOnExitTrigger
  (|CallParentFunction)
  (bind _tutorialwidgetref (Variables|Default|GetTutorialWidgetRef)
    (:then
      (Widget|RemovefromParent _tutorialwidgetref))
    (:else)))

(fn ConstructionScript
  (|CallParentFunction))