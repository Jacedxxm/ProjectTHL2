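; BP_EndTrigger is a debug trigger actor that ends the level and sends play to the credits.
; When the HL2_OffroadCar enters its sphere, it fades the player camera and audio out over FadeTime and holds the fade.
; After the fade time plus a short delay, it opens LV_Credits by object reference.
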(event OnComponentBeginOverlap(Sphere)
  (params (OverlappedComponent :type Primitive%20Component%20Object%20Reference) (OtherActor :type Actor%20Object%20Reference) (OtherComp :type Primitive%20Component%20Object%20Reference) (OtherBodyIndex :type Integer) (bFromSweep :type Boolean) (SweepResult :type Hit%20Result%20Structure%20%28by%20ref%29))
  (Utilities|Casting|CastToHL2_OffroadCar OtherActor)
  (CameraFades|StartCameraFade :self (Game|GetPlayerCameraManager 0) :ToAlpha 1.0 :Duration (Variables|Default|GetFadeTime) :bShouldFadeAudio true :bHoldWhenFinished true)
  (Utilities|FlowControl|Delay (+ (Variables|Default|GetFadeTime) 2.0))
  (Game|OpenLevel(byObjectReference) "/Game/Jace/Levels/Gyms/LV_Credits.LV_Credits"))

(event EventBeginPlay
  (|CallParentFunction) ; This node is disabled and will not be called.\nDrag off pins to build functionality.
)

(fn ConstructionScript
  (|CallParentFunction))