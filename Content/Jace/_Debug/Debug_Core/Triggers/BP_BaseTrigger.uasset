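; Base trigger Blueprint with a sphere volume that detects the player character entering and provides enter and exit hooks for child classes.
; On player entry it calls OnEnterTrigger and its dispatcher, with debug prints on both enter and exit.
; The exit hook and dispatcher fire outside the player check, and the DoOnce nodes, including the ActivateOnce branch, gate nothing.
; BeginPlay caches the player as BP_PlayerCharacter.
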(event OnComponentBeginOverlap(Sphere)
  (params (OverlappedComponent :type Primitive%20Component%20Object%20Reference) (OtherActor :type Actor%20Object%20Reference) (OtherComp :type Primitive%20Component%20Object%20Reference) (OtherBodyIndex :type Integer) (bFromSweep :type Boolean) (SweepResult :type Hit%20Result%20Structure%20%28by%20ref%29))
  ;[0.15 0.15 0.15 0.5] Enter trigger
  (if (== OtherActor (Game|GetPlayerCharacter 0))
    (Default|CallOnEnterTrigger)
    (if (Variables|Default|GetActivateOnce)
      (Utilities|FlowControl|DoOnce false
        (:Completed
          _)))
    (CallFunction|OnEnterTrigger)
    (Development|PrintString "Entered")))

(event OnComponentEndOverlap(Sphere)
  (params (OverlappedComponent :type Primitive%20Component%20Object%20Reference) (OtherActor :type Actor%20Object%20Reference) (OtherComp :type Primitive%20Component%20Object%20Reference) (OtherBodyIndex :type Integer))
  ;[0.15 0.15 0.15 0.5] Exit Trigger
  (if (== OtherActor (Game|GetPlayerCharacter 0))
    (Utilities|FlowControl|DoOnce false
      (:Completed
        _)))
  (CallFunction|OnExitTrigger)
  (Development|PrintString "Exit")
  (Default|CallOnExitTrigger))

(event Custom|On%20Enter%20Trigger
  ;[0.15 0.15 0.15 0.5] Enter trigger
)

(event Custom|On%20Exit%20Trigger
  ;[0.15 0.15 0.15 0.5] Exit Trigger
)

(event EventBeginPlay
  (bind _asbp_player_character (Utilities|Casting|CastToBP_PlayerCharacter (Game|GetPlayerCharacter 0)))
  (Variables|Default|SetPlayerCharacter _asbp_player_character))

(fn ConstructionScript)