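; BP_VisionTrigger is a trigger that plays a scripted Vortigaunt vision, warning the player about the Combine and directing them to a ship.
; It extends a parent trigger and stays inactive until the referenced lever's tower-activation event sets CanBeTriggered.
; On entry, it overlays a vision widget and plays two timed voice and HUD dialogue lines, swapping the eye material midway.
; It then clears both, leaving CanBeTriggered set.
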(event Custom|SetCanBeTriggered
  (Variables|Default|SetbCanBeTriggered true))

(event EventBeginPlay
  (|CallParentFunction)
  (EventDispatchers|BindEventtoOnTowerLeverActivated (Variables|Default|GetLeverRef) (delegate Custom|SetCanBeTriggered)))

(event EventOnEnterTrigger
  (bind _playercharacter (Variables|Default|GetPlayerCharacter))
  (bind _playercharacter_2 (Variables|Default|GetPlayerCharacter))
  (bind _playerattributeshud (Variables|/Game/FirstPerson/Blueprints/BP_PlayerCharacter.BP_PlayerCharacter_C|GetPlayerAttributesHUD _playercharacter_2))
  (|CallParentFunction)
  (if (Variables|Default|GetbCanBeTriggered)
    (bind _returnvalue (UserInterface|CreateWidget "/Game/Jace/_Debug/Debug_Core/UserInterface/WBP_VortigauntDialogue.WBP_VortigauntDialogue_C" (Game|GetPlayerController 0)))
    (bind _output_get (Variables|Default|SetVisionWidget _returnvalue))
    (UserInterface|Viewport|AddtoViewport _output_get -1)
    (Audio|PlaySound2D "/Game/Jace/_Debug/Debug_Core/Audio/SC_VortigauntVoice.SC_VortigauntVoice" 1.0 1.0 0.0 0 0)
    (Variables|/Script/UMG.Widget|SetVisibility (Variables|/Game/Jace/_Debug/Debug_Core/UserInterface/WBP_HUD.WBP_HUD_C|GetDialogueText _playerattributeshud) "Visible")
    (Default|TriggerDialogue _playerattributeshud "They’re coming for you, the Combine… they’re here… they’ve taken prisoners…")
    (Utilities|FlowControl|Delay 3.0)
    (Audio|PlaySound2D "/Game/Jace/_Debug/Debug_Core/Audio/SC_VortigauntVoice.SC_VortigauntVoice" 1.0 1.0 0.0 0 0)
    (Default|TriggerDialogue (Variables|/Game/FirstPerson/Blueprints/BP_PlayerCharacter.BP_PlayerCharacter_C|GetPlayerAttributesHUD (Variables|Default|GetPlayerCharacter)) "Contact the base… Then….Meet me at the ship… I’m northwest, you’ll have to… jump…")
    (Class|Image|SetBrushfromMaterial (Variables|/Game/Jace/_Debug/Debug_Core/UserInterface/WBP_VortigauntDialogue.WBP_VortigauntDialogue_C|GetVision (Variables|Default|GetVisionWidget)) "/Game/Art/2D/Texturres/VortigauntDialogue/MM_VortigauntEyeUI1.MM_VortigauntEyeUI1")
    (Utilities|FlowControl|Delay 4.0)
    (Variables|/Script/UMG.Widget|SetVisibility (Variables|/Game/Jace/_Debug/Debug_Core/UserInterface/WBP_HUD.WBP_HUD_C|GetDialogueText (Variables|/Game/FirstPerson/Blueprints/BP_PlayerCharacter.BP_PlayerCharacter_C|GetPlayerAttributesHUD _playercharacter)) "Hidden")
    (Default|TriggerDialogue (Variables|/Game/FirstPerson/Blueprints/BP_PlayerCharacter.BP_PlayerCharacter_C|GetPlayerAttributesHUD _playercharacter))
    (Widget|RemovefromParent (Variables|Default|GetVisionWidget))))

(fn ConstructionScript
  (|CallParentFunction))