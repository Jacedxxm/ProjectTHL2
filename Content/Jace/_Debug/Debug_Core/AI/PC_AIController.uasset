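; Enemy AI controller that runs the possessed BP_BaseEnemy's behavior tree and starts it in the Patrol state.
; Perception updates are sorted by sense and write state, target and point of interest to the Blackboard.
; Sighting the player during Patrol or Investigation triggers Attacking.
; Hearing sets Investigation from any state, bypassing the unused HandleSensedSound check, while damage only prints debug text.
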(event OnPerceptionUpdated(AIPerception)
  (params (UpdatedActors :type Array%20of%20Actor%20Object%20References))
  (for _array_element UpdatedActors
    (Utilities|FlowControl|Sequence
      (:then_0
        (bind _sensed (CallFunction|CanSenseActor _array_element "NewEnumerator1"))
        (if _sensed
          (CallFunction|HandleSensedSight _array_element)
          (Development|PrintString "Sensed Sight" true true "(R=0.100626,G=1.000000,B=0.000000,A=1.000000)")))
      (:then_1
        (bind (_sensed_2 _stimulusref) (CallFunction|CanSenseActor _array_element "NewEnumerator2"))
        (if _sensed_2
          (CallFunction|SetStatesasInvestigation (.StimulusLocation (Utilities|Struct|BreakAIStimulus _stimulusref)))
          (Development|PrintString "Sensed Hearing" true true "(R=1.000000,G=0.769687,B=0.000000,A=1.000000)")))
      (:then_2
        (bind _sensed_3 (CallFunction|CanSenseActor _array_element "NewEnumerator3"))
        (if _sensed_3
          (Development|PrintString "Sensed Damaged" true true "(R=1.000000,G=0.000000,B=0.641820,A=1.000000)")
          (Development|PrintString "Hello"))))))

(event EventPossess
  (params (PossessedPawn :type Pawn%20Object%20Reference))
  (bind _output_get (Variables|Default|SetPossesedPawn PossessedPawn))
  (bind _asbp_base_enemy (Utilities|Casting|CastToBP_BaseEnemy _output_get))
  (AI|RunBehaviorTree (Variables|/Game/Jace/_Debug/Debug_Core/AI/BaseEnemy/BP_BaseEnemy.BP_BaseEnemy_C|GetBehaviorTree _asbp_base_enemy))
  (CallFunction|SetStatesasPatrol))

(fn ConstructionScript)

(fn SetStatesasPatrol
  (AI|Components|Blackboard|SetValueasEnum (Variables|Default|GetBlackboard) (Variables|Default|GetStateKeyName) (Utilities|Enum|LiteralenumE_AIStates "NewEnumerator0")))

(fn SetStatesasAttacking
  (params (AttackTarget :type Actor%20Object%20Reference))
  (AI|Components|Blackboard|SetValueasObject (Variables|Default|GetBlackboard) (Variables|Default|GetAttackTargetKeysName) AttackTarget)
  (AI|Components|Blackboard|SetValueasEnum (Variables|Default|GetBlackboard) (Variables|Default|GetStateKeyName) (Utilities|Enum|LiteralenumE_AIStates "NewEnumerator5")))

(fn CanSenseActor
  (params (Actor :type Actor%20Object%20Reference) (Sense :type E_AISense%20Enum :default "NewEnumerator0"))
  (bind _info (Class|AIPerceptionComponent|GetActorsPerception (Variables|Default|GetAIPerception) Actor))
  (for _array_element (.lastsensedstimuli _info)
    (bind _returnvalue (Class|AIPerceptionSystem|GetSenseClassforStimulus _array_element))
    (if (== _returnvalue (Utilities|Select :Index Sense :NewEnumerator0 0 :NewEnumerator1 "/Script/AIModule.AISense_Sight" :NewEnumerator2 "/Script/AIModule.AISense_Hearing" :NewEnumerator3 "/Script/AIModule.AISense_Damage"))
      (return (.bSuccessfullySensed (Utilities|Struct|BreakAIStimulus _array_element)) _array_element))))

(fn HandleSensedSight
  (params (Actor :type Actor%20Object%20Reference))
  (bind _states (CallFunction|GetCurrentState))
  (switch Utilities|FlowControl|Switch|SwitchonE_AIStates _states
    (:NewEnumerator0
      _)
    (:NewEnumerator3
      _))
  (if (== Actor (Game|GetPlayerCharacter 0))
    (CallFunction|SetStatesasAttacking Actor)))

(fn GetCurrentState
  (return (Utilities|Enum|ByteToEnumE_AIStates (Class|BlackboardComponent|GetValueasEnum (Variables|Default|GetBlackboard) (Variables|Default|GetStateKeyName)))))

(fn HandleSensedSound
  (params (Location :type Vector))
  (bind _states (CallFunction|GetCurrentState))
  (switch Utilities|FlowControl|Switch|SwitchonE_AIStates _states
    (:NewEnumerator0
      _)
    (:NewEnumerator3
      _))
  (CallFunction|SetStatesasInvestigation Location))

(fn SetStatesasInvestigation
  (params (Location :type Vector))
  (AI|Components|Blackboard|SetValueasEnum (Variables|Default|GetBlackboard) (Variables|Default|GetStateKeyName) (Utilities|Enum|LiteralenumE_AIStates "NewEnumerator3"))
  (AI|Components|Blackboard|SetValueasVector (Variables|Default|GetBlackboard) (Variables|Default|GetPointOfInterestKeyName) Location))