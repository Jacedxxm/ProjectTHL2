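; BP_Enemy_Guard is a guard enemy Blueprint that draws and sheathes a sword and exposes its patrol route.
; Wielding plays an unsheath montage, spawns a melee weapon on a montage notify and attaches it to the right-hand socket.
; Sheathing plays its montage and destroys the weapon on a notify.
; Notifies update the wielding flag, while montage completion calls the wield or sheath callbacks, with a debug print after wielding.
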(event Custom|WieldMeleeWeapon
  (bind _notifyname (Animation|Montage|PlayMontage (Variables|Character|GetMesh) "/Game/Art/3D/_Debug/Enemies/MeleeEnemy/Animations/AM_SwordUnsheath.AM_SwordUnsheath")
    (:OnCompleted
      (Default|CallOnWieldWeapon)
      (Development|PrintString "Hello"))
    (:OnNotifyBegin
      (switch name _notifyname
        (:HoldWeapon
          (bind _returnvalue (Game|SpawnActorfromClass "/Game/Jace/_Debug/Debug_Core/Weapons/Melee/BP_BaseMeleeWeapon.BP_BaseMeleeWeapon_C" (Transformation|GetActorTransform) "AlwaysSpawn" "MultiplyWithRoot" 0 0))
          (bind _output_get (Variables|Default|SetMeleeWeapon _returnvalue))
          (Transformation|AttachComponentToComponent _output_get (Variables|Character|GetMesh) "hand_rSocket" "SnapToTarget" "SnapToTarget" "SnapToTarget" true)
          (Variables|Default|SetbIsWieldingWeapon true))))))

(event Custom|SheathMeleeWeapon
  (bind _notifyname (Animation|Montage|PlayMontage (Variables|Character|GetMesh) "/Game/Art/3D/_Debug/Enemies/MeleeEnemy/Animations/AM_SwordSheath.AM_SwordSheath")
    (:OnCompleted
      (Default|CallOnSheatWeapon))
    (:OnNotifyBegin
      (switch name _notifyname
        (:DropWeapon
          (bind _meleeweapon (Variables|Default|GetMeleeWeapon)
            (:then
              (Actor|DestroyActor _meleeweapon)
              (Variables|Default|SetbIsWieldingWeapon false))
            (:else)))))))

(event EventBeginPlay)

(event Collision|EventActorBeginOverlap
  (params (OtherActor :type Actor%20Object%20Reference)))

(fn ConstructionScript
  (|CallParentFunction))

(fn GetPatrolRoute
  (return (Variables|Default|GetPatrolRoute)))