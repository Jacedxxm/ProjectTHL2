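; Base enemy character Blueprint that provides attack, movement speed and patrol route hooks.
; Attack plays a sword slash montage when wielding a weapon, otherwise a zombie attack montage, and calls OnAttackEnd on completion or interruption.
; SetMovementSpeed maps a speed state, from idle to sprinting, to the max walk speed and returns it.
; GetPatrolRoute is an empty stub here.
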(event Custom|Attack
  (if (Variables|Default|GetbIsWieldingWeapon)
    (Animation|Montage|PlayMontage (Variables|Character|GetMesh) "/Game/Art/3D/_Debug/Enemies/MeleeEnemy/Animations/AM_SwordSlash.AM_SwordSlash"
      (:OnCompleted
        _)
      (:OnInterrupted
        _))
    (Default|CallOnAttackEnd)
    (else
      (Animation|Montage|PlayMontage (Variables|Character|GetMesh) "/Game/Art/3D/Animations/Zombie/Attack/AS_FN_Manny_Zombie_Attack_SKM_UEFN_MANNY_Anim_Montage.AS_FN_Manny_Zombie_Attack_SKM_UEFN_MANNY_Anim_Montage"
        (:OnCompleted
          _)
        (:OnInterrupted
          _))
      (Default|CallOnAttackEnd))))

(fn ConstructionScript)

(fn GetPatrolRoute
  (return 0))

(fn SetMovementSpeed
  (params (Speed :type E_AIMovementSpeed%20Enum :default "NewEnumerator0"))
  (bind _output_get (Variables|/Script/Engine.CharacterMovementComponent|SetMaxWalkSpeed (Variables|Character|GetCharacterMovement) (Utilities|Select :Index Speed :NewEnumerator0 0.0 :NewEnumerator1 1.5e+02 :NewEnumerator2 3e+02 :NewEnumerator3 7.5e+02)))
  (return _output_get))