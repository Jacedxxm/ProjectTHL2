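; Base Chaos wheeled vehicle Blueprint in a debug folder that turns player Enhanced Input into driving and look control.
; Forward and backward actions both feed throttle input on trigger and completion, while steering feeds the movement component and prints its value on screen.
; Look input drives controller yaw and pitch, with player camera manager view limits set on possession.
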(event Input|EnhancedActionEvents|EnhancedInputActionIA__VehicleMove_FWD
  (params (ActionValue :type Float%20%28double-precision%29) (ElapsedSeconds :type Float%20%28double-precision%29) (TriggeredSeconds :type Float%20%28double-precision%29) (InputAction :type Input%20Action%20Object%20Reference :default "/Game/FirstPerson/Input/Vehicle_Actions/IA__VehicleMove_FWD.IA__VehicleMove_FWD"))
  (:Triggered
    (Class|ChaosVehicleMovementComponent|SetThrottleInput (Variables|Default|GetChaosWheeledVehicleMovement) ActionValue :!label _label))
  (:Completed
    (goto _label)))

(event Input|EnhancedActionEvents|EnhancedInputActionIA__VehicleMove_Steering
  (params (ActionValue :type Float%20%28double-precision%29) (ElapsedSeconds :type Float%20%28double-precision%29) (TriggeredSeconds :type Float%20%28double-precision%29) (InputAction :type Input%20Action%20Object%20Reference :default "/Game/FirstPerson/Input/Vehicle_Actions/IA__VehicleMove_Steering.IA__VehicleMove_Steering"))
  (Class|ChaosVehicleMovementComponent|SetSteeringInput (Variables|Default|GetChaosWheeledVehicleMovement) ActionValue)
  (Development|PrintString (Utilities|String|ToString(Float) ActionValue) true true "(R=0.000000,G=0.660000,B=1.000000,A=1.000000)" 0.0))

(event Input|EnhancedActionEvents|EnhancedInputActionIA__VehicleMove_BWD
  (params (ActionValue :type Float%20%28double-precision%29) (ElapsedSeconds :type Float%20%28double-precision%29) (TriggeredSeconds :type Float%20%28double-precision%29) (InputAction :type Input%20Action%20Object%20Reference :default "/Game/FirstPerson/Input/Vehicle_Actions/IA__VehicleMove_BWD.IA__VehicleMove_BWD"))
  (:Triggered
    (Class|ChaosVehicleMovementComponent|SetThrottleInput (Variables|Default|GetChaosWheeledVehicleMovement) ActionValue :!label _label))
  (:Completed
    (goto _label)))

(event Input|EnhancedActionEvents|EnhancedInputActionIA_Look
  (params (ActionValue :type Vector%202D%20Structure) (ElapsedSeconds :type Float%20%28double-precision%29) (TriggeredSeconds :type Float%20%28double-precision%29) (InputAction :type Input%20Action%20Object%20Reference :default "/Game/FirstPerson/Input/Actions/IA_Look.IA_Look"))
  (Pawn|Input|AddControllerYawInput (.x ActionValue))
  (Pawn|Input|AddControllerPitchInput (.y ActionValue)))

(event EventBeginPlay)

(event EventPossessed
  (params (NewController :type Controller%20Object%20Reference))
  (bind _returnvalue (Game|GetPlayerCameraManager 0))
  (Utilities|IsValid _returnvalue
    (:Is%20Valid
      (Variables|/Script/Engine.PlayerCameraManager|SetViewPitchMin _returnvalue -6e+01)
      (Variables|/Script/Engine.PlayerCameraManager|SetViewPitchMax _returnvalue 6e+01)
      (Variables|/Script/Engine.PlayerCameraManager|SetViewYawMin _returnvalue -9e+01)
      (Variables|/Script/Engine.PlayerCameraManager|SetViewYawMax _returnvalue 9e+01))))

(fn ConstructionScript)