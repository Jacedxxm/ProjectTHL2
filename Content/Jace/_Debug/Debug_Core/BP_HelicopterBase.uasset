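; Helicopter actor that plays a scripted takeoff and fly-away, with a trigger binding set up at BeginPlay through TriggerRef.
; StartFlying plays a Combine alarm and helicopter sound, then timelines raise and rotate the mesh from its cached starting transform.
; When the lift finishes, a third timeline moves the mesh along relative X, and the actor destroys itself after a delay.
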(event Custom|StartFlying
  (Audio|PlaySound2D "/Game/Jace/_Debug/Debug_Core/Audio/CombineAlaram/SC_CombineAlarm.SC_CombineAlarm" 1.0 1.0 0.0 0 0)
  (Audio|PlaySoundatLocation "/Game/Jace/_Debug/Debug_Core/Audio/SC_Helicopter.SC_Helicopter" (Transformation|GetActorLocation) "0, 0, 0" 1.0 1.0 0.0 0 0 0 0)
  (bind _alpha_1 (Timeline|FlyingAnimation PlayFromStart)
    (:Update
      (Transformation|SetRelativeLocation (Variables|Default|GetMesh) (Math|Vector|Lerp(Vector) (Variables|Default|GetStartingLocation) (Math|Vector|MakeVector (.x (Variables|Default|GetStartingLocation)) (.y (Variables|Default|GetStartingLocation)) (+ (.z (Variables|Default|GetStartingLocation)) 5e+02)) _alpha_1) false false)
      (CallFunction|SetFlyingRotation))
    (:Finished
      (CallFunction|Fly)
      (Variables|Default|SetStartingLocation (Math|Vector|Lerp(Vector) (Variables|Default|GetStartingLocation) (Math|Vector|MakeVector (.x (Variables|Default|GetStartingLocation)) (.y (Variables|Default|GetStartingLocation)) (+ (.z (Variables|Default|GetStartingLocation)) 5e+02)) _alpha_1))
      (Utilities|FlowControl|Delay 7.0)
      (Utilities|IsValid self
        (:Is%20Valid
          (Actor|DestroyActor))))))

(event Custom|SetFlyingRotation
  (bind _alpha_2 (Timeline|RotationAnimation Play)
    (:Update
      (Transformation|SetRelativeRotation (Variables|Default|GetMesh) (Math|Rotator|Lerp(Rotator) (Variables|Default|GetStartingRotation) "-15.000000,0.000000,0.000000" _alpha_2) false false))))

(event Custom|Fly
  (bind _startinglocation (Variables|Default|GetStartingLocation))
  (bind _alpha_3 (Timeline|FlyAnimation Play)
    (:Update
      (Transformation|SetRelativeLocation (Variables|Default|GetMesh) (Math|Vector|Lerp(Vector) _startinglocation (+ _startinglocation "10000.000000,0.000000,0.000000") _alpha_3) false false))))

(event EventBeginPlay
  (Variables|Default|SetStartingLocation (Variables|/Script/Engine.SceneComponent|GetRelativeLocation (Variables|Default|GetMesh)))
  (Variables|Default|SetStartingRotation (Variables|/Script/Engine.SceneComponent|GetRelativeRotation (Variables|Default|GetMesh)))
  (EventDispatchers|BindEventtoOnEnterTrigger (Variables|Default|GetTriggerRef) (EventDispatchers|CreateEvent :!event Custom|StartFlying)))

(fn ConstructionScript)