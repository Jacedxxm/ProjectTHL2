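; Base door Blueprint in the level design debug folder that swings its static mesh open and closed on yaw.
; BeginPlay zeroes the mesh's relative rotation as the closed pose.
; Open uses a dot product of the door's forward vector and player direction to swing away from either side, then plays a timeline lerp unless already playing.
; Close reverses that timeline from the end.
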(event Custom|Open
  (Variables|Default|SetOpenRottionAngle (CallFunction|SetOpeningAngleBasedonCharacterPosition))
  (if (not (Audio|Components|Audio|IsPlaying (Variables|Default|GetOpen/Close%20Time)))
    (bind _alpha (Timeline|Open/Close%20Time Play)
      (:Update
        (Transformation|SetRelativeRotation (Variables|Default|GetStaticMesh) (Math|Rotator|MakeRotator 0.0 0.0 (Math|Float|Lerp (.yaw (Variables|Default|GetClosedRotation)) (Variables|Default|GetOpenRottionAngle) _alpha)) false false)))))

(event Custom|Close
  (bind _alpha (Timeline|Open/Close%20Time ReverseFromEnd)
    (:Update
      (Transformation|SetRelativeRotation (Variables|Default|GetStaticMesh) (Math|Rotator|MakeRotator 0.0 0.0 (Math|Float|Lerp (.yaw (Variables|Default|GetClosedRotation)) (Variables|Default|GetOpenRottionAngle) _alpha)) false false))))

(event EventBeginPlay
  (bind _output_get (Variables|Default|SetClosedRotation "0, 0, 0"))
  (Transformation|SetRelativeRotation (Variables|Default|GetStaticMesh) _output_get false false))

(fn ConstructionScript)

(fn SetOpeningAngleBasedonCharacterPosition
  (return (Math|Float|SelectFloat -9e+01 9e+01 (>= (Math|Vector|DotProduct (Math|Vector|GetUnitDirection(Vector) (Transformation|GetActorLocation) (Transformation|GetActorLocation (Game|GetPlayerCharacter 0))) (Transformation|GetActorForwardVector)) 0.0))))