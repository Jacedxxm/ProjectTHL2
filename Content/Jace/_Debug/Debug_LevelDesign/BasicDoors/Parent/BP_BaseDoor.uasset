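; Base door Blueprint, under debug level design, that swings its static mesh open and closed around yaw.
; Open picks a positive or negative 90-degree angle by dotting the door's forward vector with the direction to the player.
; Separate open and close timelines lerp yaw between closed and chosen angles, setting IsOpened when finished.
; BeginPlay resets the closed rotation and caches the player character; nothing here calls Open or Close.
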(event Custom|Open
  (Variables|Default|SetOpenRottionAngle (CallFunction|SetOpeningAngleBasedonCharacterPosition))
  (if (not (Math|Boolean|ANDBoolean (not (Variables|Default|GetbIsOpened)) (Audio|Components|Audio|IsPlaying (Variables|Default|GetOpen/Close%20Time)) (Audio|Components|Audio|IsPlaying (Variables|Default|GetCloseTime))))
    (bind _alpha (Timeline|Open/Close%20Time PlayFromStart)
      (:Update
        (Transformation|SetRelativeRotation (Variables|Default|GetStaticMesh) (Math|Rotator|MakeRotator 0.0 0.0 (Math|Float|Lerp (.yaw (Variables|Default|GetClosedRotation)) (Variables|Default|GetOpenRottionAngle) _alpha)) false false))
      (:Finished
        (Variables|Default|SetbIsOpened true)))))

(event Custom|Close
  (if (Variables|Default|GetbIsOpened)
    (if (not (and (Audio|Components|Audio|IsPlaying (Variables|Default|GetCloseTime)) (Audio|Components|Audio|IsPlaying (Variables|Default|GetOpen/Close%20Time))))
      (bind _alpha (Timeline|CloseTime PlayFromStart)
        (:Update
          (Transformation|SetRelativeRotation (Variables|Default|GetStaticMesh) (Math|Rotator|MakeRotator 0.0 0.0 (Math|Float|Lerp (Variables|Default|GetOpenRottionAngle) (.yaw (Variables|Default|GetClosedRotation)) _alpha)) false false))
        (:Finished
          (Variables|Default|SetbIsOpened false))))))

(event EventBeginPlay
  (bind _output_get (Variables|Default|SetClosedRotation "0, 0, 0"))
  (Transformation|SetRelativeRotation (Variables|Default|GetStaticMesh) _output_get false false)
  (bind _asbp_player_character (Utilities|Casting|CastToBP_PlayerCharacter (Game|GetPlayerCharacter 0)))
  (Variables|Default|SetPlayerCharacter _asbp_player_character))

(fn ConstructionScript)

(fn SetOpeningAngleBasedonCharacterPosition
  (return (Math|Float|SelectFloat -9e+01 9e+01 (>= (Math|Vector|DotProduct (Math|Vector|GetUnitDirection(Vector) (Transformation|GetActorLocation) (Transformation|GetActorLocation (Game|GetPlayerCharacter 0))) (Transformation|GetActorForwardVector)) 0.0))))