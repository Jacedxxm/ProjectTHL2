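; Parent Blueprint for basic debug level-design doors that swing a static mesh open and closed.
; BeginPlay sets the mesh to its closed rotation and caches the player character.
; Open, guarded by an IsOpened flag, plays a timeline that lerps yaw from the closed angle to a fixed 90 degrees with sweep.
; Close clears the flag and reverses that timeline; nothing here triggers either event.
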(event Custom|Open
  (if (not (Variables|Default|GetbIsOpened))
    (Variables|Default|SetbIsOpened true)
    (bind _alpha (Timeline|OpenTime PlayFromStart)
      (:Update
        (Transformation|SetRelativeRotation (Variables|Default|GetStaticMesh) (Math|Rotator|MakeRotator 0.0 0.0 (Math|Float|Lerp (.yaw (Variables|Rotators|GetCloseZAngle)) 9e+01 _alpha)) true false)))))

(event Custom|Close
  (Variables|Default|SetbIsOpened false)
  (bind _alpha (Timeline|OpenTime Reverse)
    (:Update
      (Transformation|SetRelativeRotation (Variables|Default|GetStaticMesh) (Math|Rotator|MakeRotator 0.0 0.0 (Math|Float|Lerp (.yaw (Variables|Rotators|GetCloseZAngle)) 9e+01 _alpha)) true false))))

(event EventBeginPlay
  (Transformation|SetRelativeRotation (Variables|Default|GetStaticMesh) (Variables|Rotators|GetCloseZAngle) false false)
  (bind _asbp_player_character (Utilities|Casting|CastToBP_PlayerCharacter (Game|GetPlayerCharacter 0)))
  (Variables|Default|SetPlayerCharacter _asbp_player_character))

(fn ConstructionScript)