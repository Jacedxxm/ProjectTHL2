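; BP_InteractableDoor is a debug level-design door that opens and closes through player interaction.
; On BeginPlay it runs the parent logic, then binds an event to the player character's BPCInteractionComponent.
; The DoorInteraction event uses a FlipFlop to alternate between Open and Close calls, starting with Open.
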(event Custom|DoorInteraction
  (Utilities|FlowControl|FlipFlop
    (:A
      (CallFunction|Open))
    (:B
      (CallFunction|Close))))

(event EventBeginPlay
  (|CallParentFunction)
  (EventDispatchers|BindEventtoInteraction (Variables|/Game/FirstPerson/Blueprints/BP_PlayerCharacter.BP_PlayerCharacter_C|GetBPC_InteractionComponent (Variables|Default|GetPlayerCharacter)) (EventDispatchers|CreateEvent :!event Custom|DoorInteraction)))

(fn ConstructionScript
  (|CallParentFunction))